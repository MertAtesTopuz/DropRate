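; Base interactable that shows a prompt widget and handles Tap or Hold interactions while it can still be interacted with.
; Tap resolves immediately, while Hold plays a timeline rotating the widget's cog, rewinding quickly on release or failure.
; Play rate distinguishes completed holds from rewinds.
; The interaction object decides success, which locks further interaction; the result is broadcast, and successful holds play a rotation and opacity animation.
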(event `self.ReceiveBeginPlay`
  (bind _aswbp_f (cast `/Game/Content/DevelopmentMain/YunusMain/Blueprints/UI/WBP_F` (`WidgetComponent.GetWidget` (`self.Widget`))))
  (set `self.InterractWidget` _aswbp_f)
  (if (`|EnumEquality` (`self.InterractionType`) "NewEnumerator2")
    (`Widget.SetVisibility` (`/Game/Content/DevelopmentMain/YunusMain/Blueprints/UI/WBP_F.F_Cog` (`self.InterractWidget`)) "Visible")))

(event `/Game/Content/DevelopmentMain/YunusMain/Blueprints/Interraction/BPI_Interract.ShowInterraction`
  (bind _widget (`self.Widget`))
  (if (`self.CanBeInterracted`)
    (if (`SceneComponent.bHiddenInGame` _widget)
      (`SceneComponent.SetHiddenInGame` _widget false false))))

(event `/Game/Content/DevelopmentMain/YunusMain/Blueprints/Interraction/BPI_Interract.HideInterraction`
  (bind _widget (`self.Widget`))
  (if (not (`SceneComponent.bHiddenInGame` _widget))
    (`SceneComponent.SetHiddenInGame` _widget true false)))

(event `/Game/Content/DevelopmentMain/YunusMain/Blueprints/Interraction/BPI_Interract.PressInterract`
  (if (`self.CanBeInterracted`)
    (switch `/Game/Content/DevelopmentMain/YunusMain/Data/E_InterractionType` (`self.InterractionType`)
      (:`NewEnumerator1`
        (`SceneComponent.SetHiddenInGame` (`self.Widget`) true false)
        (bind _returnvalue (message `/Game/Content/DevelopmentMain/YunusMain/Blueprints/Interraction/BPI_Interract.IsInterractionSuccessful` (`self.InterractionObject`)))
        (if _returnvalue
          (set `self.CanBeInterracted` false)
          (`self.InterractionResult` true)
          (else
            (`self.InterractionResult` false))))
      (:`NewEnumerator2`
        (`TimelineComponent.SetPlayRate` (`self.HoldInterraction`) 1.0)
        (bind (_direction _rotation) (`Timeline|HoldInterraction` :!label _label)
          (:`Update`
            (`Widget.SetRenderTransformAngle` (`/Game/Content/DevelopmentMain/YunusMain/Blueprints/UI/WBP_F.F_Cog` (`self.InterractWidget`)) (`KismetMathLibrary.Lerp` 0.0 180.0 _rotation)))
          (:`Finished`
            (if (<= (`TimelineComponent.GetPlayRate` (`self.HoldInterraction`)) 2.0)
              (bind _returnvalue_2 (message `/Game/Content/DevelopmentMain/YunusMain/Blueprints/Interraction/BPI_Interract.IsInterractionSuccessful` (`self.InterractionObject`)))
              (if _returnvalue_2
                (set `self.CanBeInterracted` false)
                (`self.InterractionResult` true)
                (bind (_direction_2 _rotation_2 _opacity) (`Timeline|HoldSuccesfull` :!via `PlayFromStart`)
                  (:`Update`
                    (`Widget.SetRenderTransformAngle` (`/Game/Content/DevelopmentMain/YunusMain/Blueprints/UI/WBP_F.F_Cog` (`self.InterractWidget`)) _rotation_2)
                    (`Widget.SetRenderOpacity` (`self.InterractWidget`) _opacity)))
                (else
                  (`self.InterractionResult` false)
                  (if (`self.CanBeInterracted`) :!label _label_2
                    (`TimelineComponent.SetPlayRate` (`self.HoldInterraction`) 5.0)
                    (goto _label :!via `Reverse`)))))))))))

(event `/Game/Content/DevelopmentMain/YunusMain/Blueprints/Interraction/BPI_Interract.ReleaseInterract`
  (goto _label_2))

(fn `IsInterractionSuccessful`
  (returns (ReturnValue :type Boolean))
  (return false))

(fn `UserConstructionScript`)