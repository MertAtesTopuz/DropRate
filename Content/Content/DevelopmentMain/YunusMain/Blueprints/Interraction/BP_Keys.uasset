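; BP_Keys is a key pickup that marks the first-person character as holding keys.
; On BeginPlay it sets itself as the interaction object of its child BP_Interractable and binds an event to that interaction's result.
; GainKey sets HasKeys on the character, notifies its UI that a key was collected, then destroys the child actor component and the pickup.
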(event `self.ReceiveBeginPlay`
  (bind _asbp_interractable (cast `/Game/Content/DevelopmentMain/YunusMain/Blueprints/Interraction/BP_Interractable` (`ChildActorComponent.ChildActor` (`self.ChildActor`))))
  (set `/Game/Content/DevelopmentMain/YunusMain/Blueprints/Interraction/BP_Interractable.InterractionObject` self _asbp_interractable)
  (add `/Game/Content/DevelopmentMain/YunusMain/Blueprints/Interraction/BP_Interractable.InterractionResult` _asbp_interractable (`|CreateDelegate` :!event `GainKey`)))

(event `GainKey`
  (params (Result :type Boolean))
  (bind _returnvalue (`GameplayStatics.GetActorOfClass` "/Game/Content/DefaultContent/FirstPerson/Blueprints/BP_FirstPersonCharacter.BP_FirstPersonCharacter_C"))
  (set `/Game/Content/DefaultContent/FirstPerson/Blueprints/BP_FirstPersonCharacter.HasKeys` true _returnvalue)
  (`/Game/Content/DevelopmentMain/YunusMain/Blueprints/UI/WBP_MainUI.KeyCollected` (`/Game/Content/DefaultContent/FirstPerson/Blueprints/BP_FirstPersonCharacter.UI` _returnvalue))
  (`ActorComponent.K2_DestroyComponent` (`self.ChildActor`))
  (`self.K2_DestroyActor`))

(fn `UserConstructionScript`)