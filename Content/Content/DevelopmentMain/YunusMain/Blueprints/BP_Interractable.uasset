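; BP_Interractable is an interaction prompt actor with a widget that can be shown, hidden and triggered by tap or hold.
; Tap hides the widget, plays a sound and calls InterractSuccesfull immediately.
; Hold rotates the WBP_F background via timeline; completion disables further interaction, signals success and plays a rotate/opacity animation.
; Release reverses the timeline at higher speed, and a play-rate check keeps that rewind from counting as success.
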(event `self.ReceiveBeginPlay`
  (bind _aswbp_f (cast `/Game/Content/DevelopmentMain/YunusMain/Blueprints/WBP_F` (`WidgetComponent.GetWidget` (`self.Widget`))))
  (set `self.InterractWidget` _aswbp_f))

(event `/Game/Content/DevelopmentMain/YunusMain/Blueprints/BPI_Interract.ShowInterractButton`
  (bind _widget (`self.Widget`))
  (if (`self.CanBeInterracted`)
    (if (`SceneComponent.bHiddenInGame` _widget)
      (`SceneComponent.SetHiddenInGame` _widget false false))))

(event `/Game/Content/DevelopmentMain/YunusMain/Blueprints/BPI_Interract.HideInterractButton`
  (bind _widget (`self.Widget`))
  (if (not (`SceneComponent.bHiddenInGame` _widget))
    (`SceneComponent.SetHiddenInGame` _widget true false)))

(event `/Game/Content/DevelopmentMain/YunusMain/Blueprints/BPI_Interract.PressInterract`
  (if (`self.CanBeInterracted`)
    (switch `/Game/Content/DevelopmentMain/YunusMain/Data/E_InterractionType` (`self.InterractionType`)
      (:`NewEnumerator1`
        (`SceneComponent.SetHiddenInGame` (`self.Widget`) true false)
        (`GameplayStatics.PlaySound2D` "/Engine/EditorSounds/Notifications/CompileSuccess.CompileSuccess" 1.0 1.0 0.0 null null)
        (`self.InterractSuccesfull`))
      (:`NewEnumerator2`
        (`TimelineComponent.SetPlayRate` (`self.HoldInterraction`) 1.0)
        (bind (_direction _rotation) (`Timeline|HoldInterraction` :!label _label)
          (:`Update`
            (`Widget.SetRenderTransformAngle` (`/Game/Content/DevelopmentMain/YunusMain/Blueprints/WBP_F.F_Background` (`self.InterractWidget`)) (`KismetMathLibrary.Lerp` 0.0 180.0 _rotation)))
          (:`Finished`
            (if (<= (`TimelineComponent.GetPlayRate` (`self.HoldInterraction`)) 2.0)
              (set `self.CanBeInterracted` false)
              (`GameplayStatics.PlaySound2D` "/Engine/EditorSounds/Notifications/CompileSuccess.CompileSuccess" 1.0 1.0 0.0 null null)
              (`self.InterractSuccesfull`)
              (bind (_direction_2 _rotation_2 _opacity) (`Timeline|HoldSuccesfull` :!via `PlayFromStart`)
                (:`Update`
                  (`Widget.SetRenderTransformAngle` (`/Game/Content/DevelopmentMain/YunusMain/Blueprints/WBP_F.F_Background` (`self.InterractWidget`)) _rotation_2)
                  (`Widget.SetRenderOpacity` (`self.InterractWidget`) _opacity))))))))))

(event `/Game/Content/DevelopmentMain/YunusMain/Blueprints/BPI_Interract.ReleaseInterract`
  (if (`self.CanBeInterracted`)
    (`TimelineComponent.SetPlayRate` (`self.HoldInterraction`) 5.0)
    (goto _label :!via `Reverse`)))

(fn `UserConstructionScript`)