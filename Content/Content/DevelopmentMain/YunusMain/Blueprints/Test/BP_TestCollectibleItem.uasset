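; Test collectible item actor that the first-person player picks up into their inventory through a child BP_Interractable actor.
; On BeginPlay it registers itself as that child's interaction object and binds to its interaction result.
; IsInterractionSuccessful reports whether the player's inventory is below its hardcoded limit.
; A successful result plays a sound and destroys the item if collected, while failure plays a sound and the inventory-full UI animation.
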(event `self.ReceiveBeginPlay`
  (`|ExecutionSequence`
    (:`then_0`
      (bind _asbp_first_person_character (cast `/Game/Content/DefaultContent/FirstPerson/Blueprints/BP_FirstPersonCharacter` (`GameplayStatics.GetPlayerCharacter` 0)))
      (set `self.Player` _asbp_first_person_character))
    (:`then_1`
      (bind _asbp_interractable (cast `/Game/Content/DevelopmentMain/YunusMain/Blueprints/Interraction/BP_Interractable` (`ChildActorComponent.ChildActor` (`self.ChildActor`))))
      (set `/Game/Content/DevelopmentMain/YunusMain/Blueprints/Interraction/BP_Interractable.InterractionObject` self _asbp_interractable)
      (add `/Game/Content/DevelopmentMain/YunusMain/Blueprints/Interraction/BP_Interractable.InterractionResult` _asbp_interractable (`|CreateDelegate` :!event `CollectItem`)))))

(event `CollectItem`
  (params (Result :type Boolean))
  (if Result
    (`GameplayStatics.SpawnSound2D` "/Engine/EditorSounds/Notifications/CompileSuccess.CompileSuccess" 1.0 1.0 0.0 null)
    (bind _returnvalue (`/Game/Content/DefaultContent/FirstPerson/Blueprints/BP_FirstPersonCharacter.CollectItem` (`self.Player`) (`self.Item Data`)))
    (if _returnvalue
      (`self.K2_DestroyActor`))
    (else
      (`GameplayStatics.SpawnSound2D` "/Engine/EditorSounds/Notifications/CompileFailed.CompileFailed" 1.0 1.0 0.0 null)
      (`/Game/Content/DevelopmentMain/YunusMain/Blueprints/UI/WBP_MainUI.PlayInventoryFullAnimation` (`/Game/Content/DefaultContent/FirstPerson/Blueprints/BP_FirstPersonCharacter.UI` (`self.Player`))))))

(fn `IsInterractionSuccessful`
  (returns (ReturnValue :type Boolean))
  (bind _asbp_first_person_character (cast `/Game/Content/DefaultContent/FirstPerson/Blueprints/BP_FirstPersonCharacter` (`GameplayStatics.GetPlayerCharacter` 0)))
  (return (<= (`KismetArrayLibrary.Array_Length` (`/Game/Content/DefaultContent/FirstPerson/Blueprints/BP_FirstPersonCharacter.Inventory` _asbp_first_person_character)) 3)))

(fn `UserConstructionScript`)