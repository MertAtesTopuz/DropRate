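; BP_TestItemHold is a test actor that exercises the BP_Interractable interaction system through a child actor.
; On BeginPlay it casts the child actor to BP_Interractable, sets itself as the interaction object and binds to the interaction result.
; The Interraction event plays a 2D success or failure sound based on the result.
; IsInterractionSuccessful is a stub that always returns false.
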(event `self.ReceiveBeginPlay`
  (bind _asbp_interractable (cast `/Game/Content/DevelopmentMain/YunusMain/Blueprints/Interraction/BP_Interractable` (`ChildActorComponent.ChildActor` (`self.ChildActor`))))
  (set `/Game/Content/DevelopmentMain/YunusMain/Blueprints/Interraction/BP_Interractable.InterractionObject` self _asbp_interractable)
  (add `/Game/Content/DevelopmentMain/YunusMain/Blueprints/Interraction/BP_Interractable.InterractionResult` _asbp_interractable (`|CreateDelegate` :!event `Interraction`)))

(event `Interraction`
  (params (Result :type Boolean))
  (if Result
    (`GameplayStatics.SpawnSound2D` "/Engine/EditorSounds/Notifications/CompileSuccess.CompileSuccess" 1.0 1.0 0.0 null)
    (else
      (`GameplayStatics.SpawnSound2D` "/Engine/EditorSounds/Notifications/CompileFailed.CompileFailed" 1.0 1.0 0.0 null))))

(fn `IsInterractionSuccessful`
  (returns (ReturnValue :type Boolean))
  (return false))

(fn `UserConstructionScript`)