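; BP_TestItemPlacement is a test interactable spot where the player can place a specific key item.
; On BeginPlay it binds to the first-person character's UpdateHand event to track hand changes.
; When the selected item's mesh matches KeyItem and this actor is the player's current interactable, it shows that mesh with a preview material, otherwise clearing it.
; IsInterractionSuccessful always returns true.
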(event `self.ReceiveBeginPlay`
  (bind _asbp_first_person_character (cast `/Game/Content/DefaultContent/FirstPerson/Blueprints/BP_FirstPersonCharacter` (`GameplayStatics.GetPlayerCharacter` 0)))
  (bind _output_get (set `self.Player` _asbp_first_person_character))
  (add `/Game/Content/DefaultContent/FirstPerson/Blueprints/BP_FirstPersonCharacter.UpdateHand` _output_get (`|CreateDelegate` :!event `HandUpdated`)))

(event `HandUpdated`
  (if (`self.PlayerHasKeyItem`)
    (`/Game/Content/DevelopmentMain/YunusMain/Blueprints/Interraction/BPI_Interract.ShowInterraction`)
    (else
      (`/Game/Content/DevelopmentMain/YunusMain/Blueprints/Interraction/BPI_Interract.HideInterraction`))))

(event `/Game/Content/DevelopmentMain/YunusMain/Blueprints/Interraction/BPI_Interract.ShowInterraction`
  (bind _sm_keyitem (`self.SM_KeyItem`))
  (if (`self.PlayerHasKeyItem`)
    (`StaticMeshComponent.SetStaticMesh` _sm_keyitem (`self.KeyItem`))
    (`PrimitiveComponent.SetMaterial` _sm_keyitem 0 "/Game/Content/DevelopmentMain/YunusMain/Assets/M_ItemPreview.M_ItemPreview")))

(event `/Game/Content/DevelopmentMain/YunusMain/Blueprints/Interraction/BPI_Interract.HideInterraction`
  (`StaticMeshComponent.SetStaticMesh` (`self.SM_KeyItem`) null))

(fn `IsInterractionSuccessful`
  (returns (ReturnValue :type Boolean))
  (return true))

(fn `PlayerHasKeyItem`
  (returns (ReturnValue :type Boolean))
  (return (and (== (`self.KeyItem`) (`.Mesh_7_F7BDD69646A74E31BED417B1D1DC6DD5` (break `/Game/Content/DevelopmentMain/YunusMain/Data/ST_ItemData` (`/Game/Content/DefaultContent/FirstPerson/Blueprints/BP_FirstPersonCharacter.SelectedItem` (`self.Player`))))) (== (`/Game/Content/DefaultContent/FirstPerson/Blueprints/BP_FirstPersonCharacter.Interractable` (`self.Player`)) self))))

(fn `UserConstructionScript`)