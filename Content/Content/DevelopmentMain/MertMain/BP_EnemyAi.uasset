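; BP_EnemyAi is the doll monster enemy character, providing attack, damage, patrol route, perception and speed functions for its AI.
; During attacks, a looping timer sphere-traces at the right palm socket and deals damage through an interface message until one hit succeeds.
; A lethal hit triggers a jumpscare that takes the camera, hides the player and freezes time when the montage ends.
; Any damage to the monster sets the OnJumpscare blackboard key and plays damage, then death montages.
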(event `TakeDamage`
  (`BlackboardComponent.SetValueAsBool` (`AIBlueprintHelperLibrary.GetBlackboard` null) "OnJumpscare" true)
  (`|PlayMontage` (`self.Mesh`) "/Game/Content/ArtMain/AtaMain/Characters/Basic_Enemy1/Animations/doll_monster_damage_Montage.doll_monster_damage_Montage"
    (:`OnCompleted`
      (`|PlayMontage` (`self.Mesh`) "/Game/Content/ArtMain/AtaMain/Characters/Basic_Enemy1/Animations/doll_monster_death_Montage.doll_monster_death_Montage"))))

(event `JumpscareAnim`
  (`BlackboardComponent.SetValueAsBool` (`AIBlueprintHelperLibrary.GetBlackboard` null) "OnJumpscare" true)
  (`PlayerController.SetViewTargetWithBlend` (`GameplayStatics.GetPlayerController` 0) self 0.5 "VTBlend_Linear" 0.0 false)
  (`|PlayMontage` (`self.Mesh`) "/Game/Content/ArtMain/AtaMain/Characters/Basic_Enemy1/Animations/doll_monster_QTE_Montage.doll_monster_QTE_Montage"
    (:`then`
      (`self.SetActorHiddenInGame` (`GameplayStatics.GetPlayerCharacter` 0) true))
    (:`OnCompleted`
      (`GameplayStatics.SetGlobalTimeDilation` 0.0))))

(event `Attack`
  (`|PlayMontage` (`self.Mesh`) "/Game/Content/ArtMain/AtaMain/Characters/Basic_Enemy1/Animations/doll_monster_attack1_Montage.doll_monster_attack1_Montage"
    (:`OnCompleted`
      _)
    (:`OnInterrupted`
      _))
  (`self.OnAttackEnd`))

(fn `AttackTrace`
  (bind _returnvalue (`SceneComponent.GetSocketLocation` (`self.Mesh`) "DEF-palm_01_R"))
  (if (`self.CanHit`)
    (bind _outhits (`KismetSystemLibrary.SphereTraceMulti` :`Start` _returnvalue :`End` _returnvalue :`Radius` 15.0 :`TraceChannel` "TraceTypeQuery1" :`DrawDebugType` "ForDuration"))
    (for _array_element _outhits
      (bind (_succesfull _remaninghealth) (message `/Game/Content/DevelopmentMain/YunusMain/Blueprints/Player/BPI_Damage.DealDamage` (`.HitActor` (`GameplayStatics.BreakHitResult` _array_element)) 1))
      (if _succesfull
        (`|ExecutionSequence`
          (:`then_0`
            (break))
          (:`then_1`
            (`self.EndAttackTrace`)
            (if (<= _remaninghealth 0)
              (`self.JumpscareAnim`))))))))

(fn `DamageEnemy`
  (returns (Hit :type Boolean))
  (`self.TakeDamage`)
  (return true))

(fn `DealDamage`
  (params (DamageAmount :type Integer))
  (returns (Succesfull :type Boolean) (RemaningHealth :type Integer))
  (return false 0))

(fn `EndAttackTrace`
  (`KismetSystemLibrary.K2_ClearAndInvalidateTimerHandle` (`self.AttackTraceTimer`))
  (set `self.CanHit` false))

(fn `GetPatrolRoute`
  (returns (PatrolRoute :type "/Game/Content/DevelopmentMain/MertMain/BP_PatrolRoute Object Reference"))
  (return (`self.PatrolRoute`)))

(fn `SetInvestigateValue`
  (params (Value :type "/Game/Content/DevelopmentMain/MertMain/Enum/E_InvestigateValue Enum" :default "NewEnumerator0"))
  (bind _asaic_enemy_base (cast `/Game/Content/DevelopmentMain/MertMain/AIController/AIC_EnemyBase` (`AIBlueprintHelperLibrary.GetAIController` self)))
  (switch `/Game/Content/DevelopmentMain/MertMain/Enum/E_InvestigateValue` Value
    (:`NewEnumerator0`
      (`/Game/Content/DevelopmentMain/MertMain/AIController/AIC_EnemyBase.SetDefeultPerception` _asaic_enemy_base))
    (:`NewEnumerator1`
      (`/Game/Content/DevelopmentMain/MertMain/AIController/AIC_EnemyBase.SetInvestigatePerception` _asaic_enemy_base)))
  (return))

(fn `SetMovementSpeed`
  (params (Speed :type "/Game/Content/DevelopmentMain/MertMain/Enum/E_MovementSpeed Enum" :default "NewEnumerator0"))
  (returns (SpeedValue :type "Float (double-precision)"))
  (bind _output_get (set `CharacterMovementComponent.MaxWalkSpeed` (select `/Game/Content/DevelopmentMain/MertMain/Enum/E_MovementSpeed` Speed :`NewEnumerator1` 100.0 :`NewEnumerator2` 300.0 :`NewEnumerator3` 500.0 :!type "Float (single-precision)") (`self.CharacterMovement`)))
  (return _output_get))

(fn `StartAttackTrace`
  (bind _returnvalue (`KismetSystemLibrary.K2_SetTimerDelegate` (`|CreateDelegate` :!event `AttackTrace`) 0.01 true true))
  (set `self.AttackTraceTimer` _returnvalue)
  (set `self.CanHit` true))

(fn `UserConstructionScript`)