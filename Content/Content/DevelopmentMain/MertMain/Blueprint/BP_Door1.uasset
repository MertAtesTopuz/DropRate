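; BP_Door1 is a door that swings open and closed when the player interacts with it.
; On BeginPlay it caches the player character, registers itself on its child-actor BP_Interractable and binds to that component actor's interaction result.
; A successful result drives a FlipFlop that plays or reverses a timeline setting the door's yaw.
; IsOpen toggles on every timeline update, rather than once per interaction.
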(event `self.ReceiveBeginPlay`
  (`|ExecutionSequence`
    (:`then_0`
      (bind _asbp_first_person_character (cast `/Game/Content/DefaultContent/FirstPerson/Blueprints/BP_FirstPersonCharacter` (`GameplayStatics.GetPlayerCharacter` 0)))
      (set `self.Player` _asbp_first_person_character))
    (:`then_1`
      (bind _asbp_interractable (cast `/Game/Content/DevelopmentMain/YunusMain/Blueprints/Interraction/BP_Interractable` (`ChildActorComponent.ChildActor` (`self.ChildActor`))))
      (set `/Game/Content/DevelopmentMain/YunusMain/Blueprints/Interraction/BP_Interractable.InterractionObject` self _asbp_interractable)
      (add `/Game/Content/DevelopmentMain/YunusMain/Blueprints/Interraction/BP_Interractable.InterractionResult` _asbp_interractable (`|CreateDelegate` :!event `Open/CloseDoor`)))))

(event `Open/CloseDoor`
  (params (Result :type Boolean))
  (if true
    (`/Engine/EditorBlueprintResources/StandardMacros.FlipFlop`
      (:`A`
        (bind (_direction _newtrack_0) (`Timeline|Open/CloseAnim` :!via `PlayFromStart` :!label _label)
          (:`Update`
            (`SceneComponent.K2_SetRelativeRotation` (`self.Door`) (`KismetMathLibrary.MakeRotator` 0.0 0.0 _newtrack_0) false false)
            (set `self.isOpen` (not (`self.isOpen`))))))
      (:`B`
        (goto _label :!via `Reverse`)))))

(fn `UserConstructionScript`)