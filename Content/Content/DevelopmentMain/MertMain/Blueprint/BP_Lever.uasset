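; BP_Lever is an interactable lever that operates a referenced Door.
; On BeginPlay it caches the player character and registers itself with a BP_Interractable child actor, binding to its interaction result.
; SwitchLever plays a sound and uses a FlipFlop to alternately play and reverse a timeline that rolls the lever pivot.
; When the timeline finishes, it calls OpenCloseDoor on the Door, always passing true.
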(event `self.ReceiveBeginPlay`
  (`|ExecutionSequence`
    (:`then_0`
      (bind _asbp_first_person_character (cast `/Game/Content/DefaultContent/FirstPerson/Blueprints/BP_FirstPersonCharacter` (`GameplayStatics.GetPlayerCharacter` 0)))
      (set `self.Player` _asbp_first_person_character))
    (:`then_1`
      (bind _asbp_interractable (cast `/Game/Content/DevelopmentMain/YunusMain/Blueprints/Interraction/BP_Interractable` (`ChildActorComponent.ChildActor` (`self.ChildActor`))))
      (set `/Game/Content/DevelopmentMain/YunusMain/Blueprints/Interraction/BP_Interractable.InterractionObject` self _asbp_interractable)
      (add `/Game/Content/DevelopmentMain/YunusMain/Blueprints/Interraction/BP_Interractable.InterractionResult` _asbp_interractable (`|CreateDelegate` :!event `SwitchLever`)))))

(event `SwitchLever`
  (params (Reasult :type Boolean))
  (`GameplayStatics.SpawnSound2D` "/Game/Content/DevelopmentMain/MertMain/GameSFX/LeverSfx.LeverSfx" 1.0 1.0 0.0 null)
  (`/Engine/EditorBlueprintResources/StandardMacros.FlipFlop`
    (:`A`
      (bind (_direction _newtrack_1) (`Timeline|UseLeverTimeline` :!via `PlayFromStart` :!label _label)
        (:`Update`
          (`SceneComponent.K2_SetRelativeRotation` (`self.LeverPivot`) (`KismetMathLibrary.MakeRotator` _newtrack_1) false false))
        (:`Finished`
          (`/Game/Content/DevelopmentMain/MertMain/Blueprint/BP_Door.Open/CloseDoor` (`self.Door`) true))))
    (:`B`
      (goto _label :!via `Reverse`))))

(fn `UserConstructionScript`)