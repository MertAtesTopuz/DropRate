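; BP_InspectableItem is a placeable level-design actor the player can interact with to inspect an item.
; The construction script applies its configurable mesh and material to the in-world mesh.
; On BeginPlay it registers with its child BP_Interractable and binds to the interaction result, with its success check always returning true.
; On success it plays a sound, copies mesh and material onto the level's BP_3DNote and opens WBP_InspectUI.
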(event `self.ReceiveBeginPlay`
  (bind _asbp_interractable (cast `/Game/Content/Blueprints/Interraction/BP_Interractable` (`ChildActorComponent.ChildActor` (`self.ChildActor`))))
  (set `/Game/Content/Blueprints/Interraction/BP_Interractable.InterractionObject` self _asbp_interractable)
  (add `/Game/Content/Blueprints/Interraction/BP_Interractable.InterractionResult` _asbp_interractable (`|CreateDelegate` :!event `CreateInspectUI`)))

(event `CreateInspectUI`
  (params (Result :type Boolean))
  (if Result
    (`GameplayStatics.SpawnSound2D` (`self.InterractionSound`) 1.0 1.0 0.0 null)
    (bind _returnvalue (`GameplayStatics.GetActorOfClass` "/Game/Content/Blueprints/Player/BP_3DNote.BP_3DNote_C"))
    (bind _staticmesh (`/Game/Content/Blueprints/Player/BP_3DNote.StaticMesh` _returnvalue))
    (`StaticMeshComponent.SetStaticMesh` _staticmesh (`self.Mesh`))
    (`PrimitiveComponent.SetMaterial` _staticmesh 0 (`self.Material`))
    (bind _returnvalue_2 (`|CreateWidget` "/Game/Content/Blueprints/UI/WBP_InspectUI.WBP_InspectUI_C" (`GameplayStatics.GetPlayerController` 0)))
    (`UserWidget.AddToViewport` _returnvalue_2 0)))

(fn `IsInterractionSuccessful`
  (returns (ReturnValue :type Boolean))
  (return true))

(fn `UserConstructionScript`
  (bind _cube (`self.Cube`))
  (`StaticMeshComponent.SetStaticMesh` _cube (`self.Mesh`))
  (`PrimitiveComponent.SetMaterial` _cube 0 (`self.Material`)))