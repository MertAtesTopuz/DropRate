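; BP_ModularChain is a level design tool that builds a hanging chain of configurable length in its Construction Script.
; When ChainCount exceeds two, it stacks scaled mesh links downward from the root StaticMesh, using a FlipFlop to alternate their rotation by 90 degrees.
; A physics constraint at the midpoint of each neighboring pair joins the links.
; An optional LastMesh replaces the final link, adjusted by an offset Transform.
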(fn `UserConstructionScript`
  (locals (`L-Rings` :type "Array of StaticMeshComponent Object Reference") (`L-Index` :type Integer))
  (bind _chaincount (`self.ChainCount`))
  (bind _l_rings (`local.L-Rings`))
  (bind _output (`|GetArrayItem` (`local.L-Rings`) (`local.L-Index`)))
  (bind _output_2 (`|GetArrayItem` _l_rings (`KismetArrayLibrary.Array_LastIndex` _l_rings)))
  (bind _output_3 (`|GetArrayItem` (`local.L-Rings`) (- (`local.L-Index`) 1)))
  (`KismetArrayLibrary.Array_Add` (`local.L-Rings`) (`self.StaticMesh`))
  (if (> _chaincount 2)
    (for _index (range 1 (+ _chaincount 1))
      (set `local.L-Index` _index)
      (bind _isa (`/Engine/EditorBlueprintResources/StandardMacros.FlipFlop`)
        (:`A`
          _)
        (:`B`
          _))
      (bind _returnvalue (`AddComponent|NODE_AddStaticMeshComponent-0` :`RelativeTransform` (`KismetMathLibrary.MakeTransform` (* (0.0 0.0 -17.0) (`local.L-Index`)) (select `bool` _isa :`false` (struct :`Yaw` -90.0) :!type "Rotator Structure") (0.03 0.03 0.03))))
      (`KismetArrayLibrary.Array_Add` (`local.L-Rings`) _returnvalue)
      (bind _returnvalue_2 (`AddComponent|NODE_AddPhysicsConstraintComponent-0` :`RelativeTransform` (`KismetMathLibrary.MakeTransform` (/ (+ (`SceneComponent.RelativeLocation` _output_3) (`SceneComponent.RelativeLocation` _output)) 2.0) (struct) (0.03 0.03 0.03))))
      (`PhysicsConstraintComponent.SetConstrainedComponents` _returnvalue_2 _output_3 "None" _output "None")
      (if (== (`self.ChainCount`) (`local.L-Index`))
        (bind _lastmesh (`self.LastMesh`)
          (:`then`
            (`StaticMeshComponent.SetStaticMesh` _output_2 _lastmesh)
            (`SceneComponent.K2_SetRelativeTransform` _output_2 (`KismetMathLibrary.MakeTransform` (+ (`SceneComponent.RelativeLocation` _output_2) (.location (`self.Transform`))) (.rotation (`self.Transform`)) (* (.scale (`self.Transform`)) (0.03 0.03 0.03))) false false))
          (:`else`))))))