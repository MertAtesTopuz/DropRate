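; BP_Bookshelf is a level design tool that builds a row of bookshelf modules from an editable Objects array.
; The construction script clears and refills instanced static meshes, picking one of three variants per array entry.
; It advances along local X by half the sum of neighboring module widths, so differently sized pieces sit edge to edge.
; Right and left corner meshes cap the two ends.
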(fn `UserConstructionScript`
  (bind _objects (`self.Objects`))
  (set `self.Offset` 0.0)
  (`InstancedStaticMeshComponent.ClearInstances` (`self.ISM_Rigth_Corner`))
  (`InstancedStaticMeshComponent.ClearInstances` (`self.ISM_Left_Corner`))
  (`InstancedStaticMeshComponent.ClearInstances` (`self.ISM_Var1`))
  (`InstancedStaticMeshComponent.ClearInstances` (`self.ISM_Var2`))
  (`InstancedStaticMeshComponent.ClearInstances` (`self.ISM_Var3`))
  (for (_array_element _array_index) (`self.Objects`)
    (`InstancedStaticMeshComponent.AddInstance` (select `int` _array_element :`0` (`self.ISM_Var1`) :`1` (`self.ISM_Var2`) :`2` (`self.ISM_Var3`)) (`KismetMathLibrary.MakeTransform` (`KismetMathLibrary.MakeVector` (`self.Offset`))) false)
    (bind _returnvalue (+ _array_index 1))
    (set `self.Offset` (+ (`self.Offset`) (/ (+ (select `int` (`|GetArrayItem` _objects _array_index) :`0` 200.0 :`1` 200.0 :`2` 155.0) (`KismetMathLibrary.SelectFloat` (select `int` (`|GetArrayItem` _objects _returnvalue) :`0` 200.0 :`1` 200.0 :`2` 155.0) 0.0 (`KismetArrayLibrary.Array_IsValidIndex` _objects _returnvalue))) 2.0))))
  (`InstancedStaticMeshComponent.AddInstance` (`self.ISM_Rigth_Corner`) (`KismetMathLibrary.MakeTransform` (`KismetMathLibrary.MakeVector` (* (select `int` (`|GetArrayItem` (`self.Objects`)) :`0` 200.0 :`1` 200.0 :`2` 155.0) -0.5))) false)
  (`InstancedStaticMeshComponent.AddInstance` (`self.ISM_Left_Corner`) (`KismetMathLibrary.MakeTransform` (`KismetMathLibrary.MakeVector` (`self.Offset`))) false))