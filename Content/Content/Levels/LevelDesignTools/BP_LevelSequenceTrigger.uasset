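; Level design trigger that plays an assigned Level Sequence once when the player character overlaps it, hiding the character meanwhile.
; Two parallel delays derive from the sequence's play length.
; At the halfway point, if TriggerEnemy is set, it assigns PatrolRoute to BPEnemy, starts it and enables player input.
; At the full length it unhides the character and disables player input.
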(event `self.ReceiveActorBeginOverlap`
  (params (OtherActor :type "Actor Object Reference"))
  (bind _returnvalue (`GameplayStatics.GetPlayerController` 0))
  (bind _returnvalue_2 (`GameplayStatics.GetPlayerController` 0))
  (bind _bp_enemy (`self.BP_Enemy`))
  (if (== OtherActor (`GameplayStatics.GetPlayerCharacter` 0))
    (`/Engine/EditorBlueprintResources/StandardMacros.DoOnce` false
      (:`Completed`
        (`self.SetActorHiddenInGame` (`GameplayStatics.GetPlayerCharacter` 0) true)
        (bind (_outactor _returnvalue_3) (`LevelSequencePlayer.CreateLevelSequencePlayer` (`self.Level Sequence`)))
        (`MovieSceneSequencePlayer.Play` _returnvalue_3)
        (bind _returnvalue_4 (message `AnimationDataModel.GetPlayLength` _returnvalue_3))
        (`|ExecutionSequence`
          (:`then_0`
            (`KismetSystemLibrary.Delay` _returnvalue_4)
            (`self.SetActorHiddenInGame` (`GameplayStatics.GetPlayerCharacter` 0) false)
            (`self.DisableInput` _returnvalue_2 _returnvalue_2))
          (:`then_1`
            (`KismetSystemLibrary.Delay` (/ _returnvalue_4 2.0))
            (if (`self.TriggerEnemy`)
              (set `/Game/Content/Blueprints/Enemy/BP_EnemyAi.PatrolRoute` (`self.Patrol Route`) _bp_enemy)
              (`/Game/Content/Blueprints/Enemy/BP_EnemyAi.Start` _bp_enemy)
              (`self.EnableInput` _returnvalue _returnvalue))))))))

(fn `UserConstructionScript`)