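; BP_LevelSequenceTrigger is an overlap trigger that plays a level sequence once when the first player character enters it.
; It hides the player character, creates and plays a sequence player, then uses a delay matching the sequence length to unhide the character.
; If TriggerEnemy is set, a parallel delay assigns PatrolRoute to BPEnemy and starts it halfway through the sequence.
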(event `self.ReceiveActorBeginOverlap`
  (params (OtherActor :type "Actor Object Reference"))
  (bind _bp_enemy (`self.BP_Enemy`))
  (if (== OtherActor (`GameplayStatics.GetPlayerCharacter` 0))
    (`/Engine/EditorBlueprintResources/StandardMacros.DoOnce` false
      (:`Completed`
        (`self.SetActorHiddenInGame` (`GameplayStatics.GetPlayerCharacter` 0) true)
        (bind (_outactor _returnvalue) (`LevelSequencePlayer.CreateLevelSequencePlayer` (`self.Level Sequence`)))
        (`MovieSceneSequencePlayer.Play` _returnvalue)
        (bind _returnvalue_2 (message `AnimationDataModel.GetPlayLength` _returnvalue))
        (`|ExecutionSequence`
          (:`then_0`
            (`KismetSystemLibrary.Delay` _returnvalue_2)
            (`self.SetActorHiddenInGame` (`GameplayStatics.GetPlayerCharacter` 0) false))
          (:`then_1`
            (`KismetSystemLibrary.Delay` (/ _returnvalue_2 2.0))
            (if (`self.TriggerEnemy`)
              (set `/Game/Content/DevelopmentMain/MertMain/BP_EnemyAi.PatrolRoute` (`self.Patrol Route`) _bp_enemy)
              (`/Game/Content/DevelopmentMain/MertMain/BP_EnemyAi.Start` _bp_enemy))))))))

(fn `UserConstructionScript`)