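; BP_Ragdoll is a doll whose head the player can take as an inventory item.
; It binds RemoveHead to the interaction result of a child-actor BP_Interractable.
; If the first-person character's inventory has room, the head is collected and hidden through a dynamic material scalar on the skeletal mesh.
; Otherwise the inventory-full UI animation plays, with the grab sound playing in both cases.
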(event `self.ReceiveBeginPlay`
  (bind _asbp_interractable (cast `/Game/Content/Blueprints/Interraction/BP_Interractable` (`ChildActorComponent.ChildActor` (`self.ChildActor`))))
  (add `/Game/Content/Blueprints/Interraction/BP_Interractable.InterractionResult` _asbp_interractable (delegate `RemoveHead`)))

(event `RemoveHead`
  (params (Result :type Boolean))
  (if (<= (`KismetArrayLibrary.Array_Length` (`/Game/Content/Blueprints/Player/BP_FirstPersonCharacter.Inventory` (cast `/Game/Content/Blueprints/Player/BP_FirstPersonCharacter` (`GameplayStatics.GetPlayerCharacter` 0) :!pure true))) 3)
    (`GameplayStatics.SpawnSound2D` "/Game/Content/Assets/Sounds/SoundWaves/SW_GrabItem.SW_GrabItem" 1.0 1.0 0.0 null)
    (bind _returnvalue (`/Game/Content/Blueprints/Player/BP_FirstPersonCharacter.CollectItem` (cast `/Game/Content/Blueprints/Player/BP_FirstPersonCharacter` (`GameplayStatics.GetPlayerCharacter` 0) :!pure true) (make `/Game/Content/Blueprints/Data/ST_ItemData` "Head" "/Game/Content/Assets/Meshes/Doll_MonsterHeadBroken.Doll_MonsterHeadBroken" "/Game/Content/Assets/Textures/Item_Icons/T_Icon_Metalhead.T_Icon_Metalhead" "NewEnumerator5")))
    (if _returnvalue
      (bind _returnvalue_2 (`PrimitiveComponent.CreateDynamicMaterialInstance` (`self.SkeletalMesh`) 0 null "None"))
      (`MaterialInstanceDynamic.SetScalarParameterValue` _returnvalue_2 "HeadVisible" 0.0))
    (else
      (`GameplayStatics.SpawnSound2D` "/Game/Content/Assets/Sounds/SoundWaves/SW_GrabItem.SW_GrabItem" 1.0 1.0 0.0 null)
      (`/Game/Content/Blueprints/UI/WBP_MainUI.PlayInventoryFullAnimation` (`/Game/Content/Blueprints/Player/BP_FirstPersonCharacter.UI` (cast `/Game/Content/Blueprints/Player/BP_FirstPersonCharacter` (`GameplayStatics.GetPlayerCharacter` 0) :!pure true))))))

(fn `UserConstructionScript`)