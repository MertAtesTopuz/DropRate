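; Witch statue puzzle actor that hands out an axe and tracks a set of linked heads.
; Its child interactable triggers the pickup, which adds the axe to the player's inventory and removes the mesh, or plays an inventory-full animation.
; Head delegates feed placed and broken counters: four placed makes every head hittable, while four broken currently only prints a debug string.
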(event `self.ReceiveBeginPlay`
  (`|ExecutionSequence`
    (:`then_0`
      (bind _asbp_first_person_character (cast `/Game/Content/Blueprints/Player/BP_FirstPersonCharacter` (`GameplayStatics.GetPlayerCharacter` 0)))
      (set `self.Player` _asbp_first_person_character))
    (:`then_1`
      (bind _asbp_interractable (cast `/Game/Content/Blueprints/Interraction/BP_Interractable` (`ChildActorComponent.ChildActor` (`self.ChildActor`))))
      (set `/Game/Content/Blueprints/Interraction/BP_Interractable.InterractionObject` self _asbp_interractable)
      (add `/Game/Content/Blueprints/Interraction/BP_Interractable.InterractionResult` _asbp_interractable (`|CreateDelegate` :!event `CollectItem`)))
    (:`then_2`
      (for _array_element (`self.Heads`)
        (add `/Game/Content/Blueprints/Test/BP_HeadPlace.HeadPlaced` _array_element (`|CreateDelegate` :!event `HeadsPlaced`))
        (add `/Game/Content/Blueprints/Test/BP_HeadPlace.HeadBroken` _array_element (`|CreateDelegate` :!event `HeadsBroken`))))))

(event `CollectItem`
  (params (Result :type Boolean))
  (if (<= (`KismetArrayLibrary.Array_Length` (`/Game/Content/Blueprints/Player/BP_FirstPersonCharacter.Inventory` (`self.Player`))) 3)
    (`GameplayStatics.SpawnSound2D` null 1.0 1.0 0.0 null)
    (bind _returnvalue (`/Game/Content/Blueprints/Player/BP_FirstPersonCharacter.CollectItem` (`self.Player`) (make `/Game/Content/Blueprints/Data/ST_ItemData` "" "/Game/Content/Assets/Meshes/SM_AxeHandHeld.SM_AxeHandHeld" "/Game/Content/Assets/Textures/Item_Icons/T_Icon_Axe.T_Icon_Axe" "NewEnumerator4")))
    (if _returnvalue
      (`ActorComponent.K2_DestroyComponent` (`self.StaticMesh`)))
    (else
      (`GameplayStatics.SpawnSound2D` null 1.0 1.0 0.0 null)
      (`/Game/Content/Blueprints/UI/WBP_MainUI.PlayInventoryFullAnimation` (`/Game/Content/Blueprints/Player/BP_FirstPersonCharacter.UI` (`self.Player`))))))

(fn `HeadsBroken`
  (bind _result (`/Engine/EditorBlueprintResources/StandardMacros.IncrementInt` (`self.BrokenHeads`))
    (:`  `
      (if (>= _result 4)
        (`KismetSystemLibrary.PrintString` "b")))))

(fn `HeadsPlaced`
  (bind _result (`/Engine/EditorBlueprintResources/StandardMacros.IncrementInt` (`self.PlacedHeads`))
    (:`  `
      (if (>= _result 4)
        (for _array_element (`self.Heads`)
          (set `/Game/Content/Blueprints/Test/BP_HeadPlace.CanHit` true _array_element))
        (`KismetSystemLibrary.PrintString` "a")))))

(fn `UserConstructionScript`)