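; BP_DoorCage is a cage door actor that swings open or closed through its Open/CloseDoor event.
; A true result on a closed door plays an unlock sound and runs a timeline from the start to drive the door's relative yaw.
; A false result on an open door reverses the same timeline, and the open flag flips whenever the timeline finishes.
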(event `self.ReceiveBeginPlay`)

(event `Open/CloseDoor`
  (params (Result :type Boolean))
  (if (and Result (!= (`self.isOpen`) true))
    (`GameplayStatics.PlaySound2D` "/Game/Content/Assets/Sounds/SoundWaves/SW_UnlockWoodenDoor.SW_UnlockWoodenDoor" 1.0 1.0 0.0 null null)
    (bind (_direction _newtrack_0) (`Timeline|Open/CloseAnim` :!via `PlayFromStart` :!label _label)
      (:`Update`
        (`SceneComponent.K2_SetRelativeRotation` (`self.Door`) (`KismetMathLibrary.MakeRotator` 0.0 0.0 _newtrack_0) false false))
      (:`Finished`
        (set `self.isOpen` (not (`self.isOpen`)))))
    (elif (and (!= Result true) (!= (`self.isOpen`) false))
      (goto _label :!via `Reverse`))))

(fn `UserConstructionScript`)