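; BP_NumericLock is a six-part numeric combination lock whose parts rotate through ten digit positions.
; RotatePart animates a part's roll by 36 degrees with a timeline, using CanRotate to block overlapping turns.
; When a turn finishes, PrintCode converts each part's roll into a digit and prints the combined code.
; BeginPlay turns part 4 every two seconds, with no player input or code check.
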(event `self.ReceiveBeginPlay`
  (`KismetSystemLibrary.Delay` 2.0 :!label _label)
  (`self.RotatePart` (`self.4`))
  (goto _label))

(event `RotatePart`
  (params (RotatablePart :type "SceneComponent Object Reference"))
  (bind _relativerotation_roll (`KismetMathLibrary.BreakRotator` (`SceneComponent.RelativeRotation` RotatablePart)))
  (if (`self.CanRotate`)
    (set `self.CanRotate` false)
    (bind _output_get (set `self.CurrentRotation` _relativerotation_roll))
    (set `self.TargetRotation` (+ _output_get 36.0))
    (bind (_direction _newtrack_0) (`Timeline|TurnPart` :!via `PlayFromStart`)
      (:`Update`
        (`SceneComponent.K2_SetRelativeRotation` RotatablePart (`KismetMathLibrary.MakeRotator` (`KismetMathLibrary.Lerp` (`self.CurrentRotation`) (`self.TargetRotation`) _newtrack_0)) false false))
      (:`Finished`
        (set `self.CanRotate` true)
        (bind _password (`self.PrintCode`))
        (`KismetSystemLibrary.PrintString` _password)))))

(fn `PrintCode`
  (returns (PassWord :type String))
  (locals (`L-PassWord` :type String))
  (for _array_element (`|MakeArray` (`self.1`) (`self.2`) (`self.3`) (`self.4`) (`self.5`) (`self.6`))
    (bind _roll (.roll (`SceneComponent.RelativeRotation` _array_element)))
    (set `local.L-PassWord` (`KismetStringLibrary.Concat_StrStr` (`local.L-PassWord`) (`KismetStringLibrary.Conv_IntToString` (`KismetMathLibrary.FTrunc` (/ (select `bool` (< _roll 0.0) :`false` _roll :`true` (+ _roll 360.0) :!type "Float (single-precision)") 36.0))))))
  (return (`local.L-PassWord`)))

(fn `UserConstructionScript`)