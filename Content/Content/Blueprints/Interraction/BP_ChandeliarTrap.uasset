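; BP_ChandeliarTrap is a chandelier trap that drops to damage pawns and can be winched back up to re-arm.
; GoDown lerps Rooter to TargetLocation via timeline, sending DamageEnemyMessage to the pawn hit by a sphere trace below it each update.
; StartArming raises it, clearing Down near the top; StopArming rapidly reverses that motion.
; BeginPlay runs a timed drop, arm and drop sequence.
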(event `self.ReceiveBeginPlay`
  (`KismetSystemLibrary.Delay` 2.0)
  (`self.GoDown`)
  (`KismetSystemLibrary.Delay` 1.0)
  (`self.StartArming`)
  (`KismetSystemLibrary.Delay` 10.0)
  (`self.GoDown`))

(event `GoDown`
  (bind _returnvalue (- (`SceneComponent.K2_GetComponentLocation` (`self.Rooter`)) (0.0 0.0 200.0)))
  (if (not (`self.Down`))
    (bind (_direction _location) (`Timeline|GoDownTimeline` :!via `PlayFromStart`)
      (:`Update`
        (`SceneComponent.K2_SetRelativeLocation` (`self.Rooter`) (`KismetMathLibrary.VLerp` (0.0 0.0 0.0) (`self.TargetLocation`) _location) false false)
        (bind _outhit (`KismetSystemLibrary.SphereTraceSingleForObjects` :`Start` _returnvalue :`End` _returnvalue :`Radius` 150.0 :`ObjectTypes` (`|MakeArray` "ObjectTypeQuery3" :!type "EObjectTypeQuery Enum") :`DrawDebugType` "ForOneFrame"))
        (message `/Game/Content/Blueprints/Management/BPI_Damage.DamageEnemy` (`.HitActor` (`GameplayStatics.BreakHitResult` _outhit))))
      (:`Finished`
        (set `self.Down` true)))))

(event `StartArming`
  (if (`self.Down`)
    (`TimelineComponent.SetPlayRate` (`self.Arm`) 1.0)
    (bind (_direction _newtrack_0) (`Timeline|Arm` :!label _label)
      (:`Update`
        (`SceneComponent.K2_SetRelativeLocation` (`self.Rooter`) (`KismetMathLibrary.VLerp` (`self.TargetLocation`) (0.0 0.0 0.0) _newtrack_0) false false))
      (:`Finished`
        (if (> (.z (`SceneComponent.RelativeLocation` (`self.Rooter`))) -50.0)
          (set `self.Down` false))))))

(event `StopArming`
  (if (`self.Down`)
    (`TimelineComponent.SetPlayRate` (`self.Arm`) 6.0)
    (goto _label :!via `Reverse`)))

(fn `UserConstructionScript`)