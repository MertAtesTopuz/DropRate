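; BP_Interractable is an interaction point with a configurable box and a WBP_F prompt widget that can be shown or hidden, supporting Tap or Hold input.
; Tap asks InterractionObject whether it succeeds, reports the result and locks on success.
; Hold fills a timeline-driven bar that rewinds faster on release, using play rate to detect completion.
; Completed holds always report success, lock, and animate widget opacity, ignoring the object's answer.
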(event `self.ReceiveBeginPlay`
  (bind _aswbp_f (cast `/Game/Content/Blueprints/UI/WBP_F` (`WidgetComponent.GetWidget` (`self.Widget`))))
  (set `self.InterractWidget` _aswbp_f)
  (if (`|EnumEquality` (`self.InterractionType`) "NewEnumerator2")
    (`/Game/Content/Blueprints/UI/WBP_F.SetVersion` (`self.InterractWidget`) true)))

(event `/Game/Content/Blueprints/Management/BPI_Interract.ShowInterraction`
  (bind _widget (`self.Widget`))
  (if (`self.CanBeInterracted`)
    (if (`SceneComponent.bHiddenInGame` _widget)
      (`SceneComponent.SetHiddenInGame` _widget false false))))

(event `/Game/Content/Blueprints/Management/BPI_Interract.HideInterraction`
  (bind _widget (`self.Widget`))
  (if (not (`SceneComponent.bHiddenInGame` _widget))
    (`SceneComponent.SetHiddenInGame` _widget true false)))

(event `/Game/Content/Blueprints/Management/BPI_Interract.PressInterract`
  (if (`self.CanBeInterracted`)
    (switch `/Game/Content/Blueprints/Data/E_InterractionType` (`self.InterractionType`)
      (:`NewEnumerator1`
        (if (`self.ShouldWidgetHide`)
          (`SceneComponent.SetHiddenInGame` (`self.Widget`) true false))
        (bind _returnvalue (message `/Game/Content/Blueprints/Management/BPI_Interract.IsInterractionSuccessful` (`self.InterractionObject`)))
        (if _returnvalue
          (set `self.CanBeInterracted` false)
          (`self.InterractionResult` true)
          (else
            (`self.InterractionResult` false))))
      (:`NewEnumerator2`
        (`TimelineComponent.SetPlayRate` (`self.HoldInterraction`) 1.0)
        (bind (_direction _rotation) (`Timeline|HoldInterraction` :!label _label)
          (:`Update`
            (`ProgressBar.SetPercent` (`/Game/Content/Blueprints/UI/WBP_F.HoldBar` (`self.InterractWidget`)) (`KismetMathLibrary.Lerp` 0.0 1.0 _rotation)))
          (:`Finished`
            (if (<= (`TimelineComponent.GetPlayRate` (`self.HoldInterraction`)) 2.0)
              (bind _returnvalue_2 (message `/Game/Content/Blueprints/Management/BPI_Interract.IsInterractionSuccessful` (`self.InterractionObject`)))
              (if _returnvalue_2
                _
                (else
                  _))
              (set `self.CanBeInterracted` false)
              (`self.InterractionResult` true)
              (bind (_direction_2 _rotation_2 _opacity) (`Timeline|HoldSuccesfull` :!via `PlayFromStart`)
                (:`Update`
                  (`Widget.SetRenderOpacity` (`self.InterractWidget`) _opacity))
                (:`Finished`
                  (`ProgressBar.SetPercent` (`/Game/Content/Blueprints/UI/WBP_F.HoldBar` (`self.InterractWidget`)) 1.0))))))))))

(event `/Game/Content/Blueprints/Management/BPI_Interract.ReleaseInterract`
  (if (`self.CanBeInterracted`)
    (`TimelineComponent.SetPlayRate` (`self.HoldInterraction`) 5.0)
    (goto _label :!via `Reverse`)))

(fn `IsInterractionSuccessful`
  (returns (ReturnValue :type Boolean))
  (return false))

(fn `UserConstructionScript`
  (`BoxComponent.SetBoxExtent` (`self.Box`) (`self.BoxExtend`) true)
  (`SceneComponent.K2_SetRelativeLocation` (`self.Widget`) (`self.WidgetLocation`) false false))