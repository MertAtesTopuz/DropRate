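; BP_BreakableWood is a breakable wood obstacle that shatters the first time its DamageEnemy function is called.
; A DoOnce-guarded event destroys the actors in the SMs array, plays a 2D bat-hit sound and spawns a scaled-up Niagara wood effect at the Box, removing it after a short delay.
; DealDamage and KillEnemy are stubs that report failure, so no health is tracked.
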(event `31`
  (`/Engine/EditorBlueprintResources/StandardMacros.DoOnce` false
    (:`Completed`
      (for _array_element (`self.SMs`)
        (`/Engine/EditorBlueprintResources/StandardMacros.IsValid` _array_element
          (:`Is Valid`
            (`self.K2_DestroyActor` _array_element))))
      (`GameplayStatics.SpawnSound2D` "/Game/Content/Assets/Sounds/SoundWaves/SW_BatHit3.SW_BatHit3" 1.0 1.0 0.0 null)
      (bind _returnvalue (`NiagaraFunctionLibrary.SpawnSystemAtLocation` "/Game/Generic_Item_Destruction_FX/Visual_Effects/NiagaraSystem/NS_Wood2.NS_Wood2" (`SceneComponent.K2_GetComponentLocation` (`self.Box`)) (struct) (3.0 3.0 3.0)))
      (`KismetSystemLibrary.Delay` 1.0)
      (`ActorComponent.K2_DestroyComponent` _returnvalue))))

(fn `DamageEnemy`
  (returns (Hit :type Boolean))
  (`self.31`)
  (return false))

(fn `DealDamage`
  (params (DamageAmount :type Integer))
  (returns (Succesfull :type Boolean) (RemaningHealth :type Integer))
  (return false 0))

(fn `KillEnemy`
  (returns (Hit :type Boolean))
  (return false))

(fn `UserConstructionScript`)