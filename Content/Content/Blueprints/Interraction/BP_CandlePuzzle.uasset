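; BP_CandlePuzzle is an interaction puzzle that checks which items sit on a set of candles against known codes.
; CheckOrder appends each candle's key item mesh index within its PlacableItems to LCode, using 0 when the mesh is absent.
; It compares LCode to each entry in Codes and switches on the matching index, with no outcomes wired, then prints LCode.
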(fn `CheckOrder`
  (locals (`L-Code` :type String))
  (for _array_element (`self.Candles`)
    (bind _placableitems (`/Game/Content/Blueprints/Interraction/BP_Candles.PlacableItems` _array_element))
    (bind _staticmesh (`StaticMeshComponent.StaticMesh` (`/Game/Content/Blueprints/Interraction/BP_Candles.SM_KeyItem` _array_element)))
    (set `local.L-Code` (`KismetStringLibrary.Concat_StrStr` (`local.L-Code`) (`KismetStringLibrary.Conv_IntToString` (select `bool` (`KismetArrayLibrary.Array_Contains` _placableitems _staticmesh) :`true` (`KismetArrayLibrary.Array_Find` _placableitems _staticmesh))))))
  (for (_array_element_2 _array_index) (`self.Codes`)
    (if (`KismetStringLibrary.EqualEqual_StrStr` _array_element_2 (`local.L-Code`))
      (switch `int` _array_index)))
  (`KismetSystemLibrary.PrintString` (`local.L-Code`)))

(fn `UserConstructionScript`)