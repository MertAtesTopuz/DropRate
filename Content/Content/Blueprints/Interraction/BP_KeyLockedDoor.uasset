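; Key-locked door that swings open when the player interacts with it while holding keys.
; On BeginPlay it registers itself with its BP_Interractable child actor and binds to that actor's interaction result.
; With keys, it notifies the player UI, removes the interactable, plays an unlock sound and rotates the mesh open via a Timeline.
; Without keys, it has the UI signal that a key is required.
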(event `self.ReceiveBeginPlay`
  (bind _asbp_interractable (cast `/Game/Content/Blueprints/Interraction/BP_Interractable` (`ChildActorComponent.ChildActor` (`self.ChildActor`))))
  (set `/Game/Content/Blueprints/Interraction/BP_Interractable.InterractionObject` self _asbp_interractable)
  (add `/Game/Content/Blueprints/Interraction/BP_Interractable.InterractionResult` _asbp_interractable (`|CreateDelegate` :!event `TryOpenDoor`)))

(event `TryOpenDoor`
  (params (Result :type Boolean))
  (bind _returnvalue (`GameplayStatics.GetActorOfClass` "/Game/Content/Blueprints/Player/BP_FirstPersonCharacter.BP_FirstPersonCharacter_C"))
  (if (`/Game/Content/Blueprints/Player/BP_FirstPersonCharacter.HasKeys` _returnvalue)
    (bind _returnvalue_2 (`GameplayStatics.GetActorOfClass` "/Game/Content/Blueprints/Player/BP_FirstPersonCharacter.BP_FirstPersonCharacter_C"))
    (`/Game/Content/Blueprints/UI/WBP_MainUI.KeyUsed` (`/Game/Content/Blueprints/Player/BP_FirstPersonCharacter.UI` _returnvalue_2))
    (`ActorComponent.K2_DestroyComponent` (`self.ChildActor`))
    (`GameplayStatics.PlaySound2D` "/Game/Content/Assets/Sounds/SoundWaves/SW_UnlockWoodenDoor.SW_UnlockWoodenDoor" 1.0 1.0 0.0 null null)
    (bind (_direction _newtrack_0) (`Timeline|Timeline` :!via `PlayFromStart`)
      (:`Update`
        (`SceneComponent.K2_SetRelativeRotation` (`self.StaticMesh`) (`KismetMathLibrary.MakeRotator` 0.0 0.0 (`KismetMathLibrary.Lerp` 0.0 90.0 _newtrack_0)) false false)))
    (else
      (bind _returnvalue_3 (`GameplayStatics.GetActorOfClass` "/Game/Content/Blueprints/Player/BP_FirstPersonCharacter.BP_FirstPersonCharacter_C"))
      (`/Game/Content/Blueprints/UI/WBP_MainUI.KeyRequired` (`/Game/Content/Blueprints/Player/BP_FirstPersonCharacter.UI` _returnvalue_3)))))

(fn `UserConstructionScript`)