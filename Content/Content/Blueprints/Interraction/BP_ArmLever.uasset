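; Hold-to-use arm lever that arms the BP_ChandeliarTrap chandelier while it is down.
; A child BP_Interractable supplies press and release events, which start or stop arming and play or reverse a timeline rotating the lever pivot.
; When the timeline finishes, it reloads BP_DropLever and disables its own interaction if the chandelier is still down.
; Its Reload event resets the pivot and re-enables interaction.
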(event `self.ReceiveBeginPlay`
  (`|ExecutionSequence`
    (:`then_0`
      (bind _asbp_first_person_character (cast `/Game/Content/Blueprints/Player/BP_FirstPersonCharacter` (`GameplayStatics.GetPlayerCharacter` 0)))
      (set `self.Player` _asbp_first_person_character)
      (bind _returnvalue (`GameplayStatics.GetActorOfClass` "/Game/Content/Blueprints/Interraction/BP_ChandeliarTrap.BP_ChandeliarTrap_C"))
      (set `self.Chandeliar` _returnvalue))
    (:`then_1`
      (bind _asbp_interractable (cast `/Game/Content/Blueprints/Interraction/BP_Interractable` (`ChildActorComponent.ChildActor` (`self.ChildActor`))))
      (set `self.As BP Interractable` _asbp_interractable)
      (set `/Game/Content/Blueprints/Interraction/BP_Interractable.InterractionObject` self _asbp_interractable)
      (add `/Game/Content/Blueprints/Interraction/BP_Interractable.InterractionResult` _asbp_interractable (`|CreateDelegate` :!event `SwitchLever`))
      (add `/Game/Content/Blueprints/Interraction/BP_Interractable.Pressed` _asbp_interractable (`|CreateDelegate` :!event `AA`))
      (add `/Game/Content/Blueprints/Interraction/BP_Interractable.Relesad` _asbp_interractable (`|CreateDelegate` :!event `BB`)))))

(event `SwitchLever`
  (params (Reasult :type Boolean)))

(event `AA`
  (if (`/Game/Content/Blueprints/Interraction/BP_ChandeliarTrap.Down` (`self.Chandeliar`))
    (`/Game/Content/Blueprints/Interraction/BP_ChandeliarTrap.StartArming` (`self.Chandeliar`))
    (bind (_direction _newtrack_1) (`Timeline|UseLeverTimeline` :!via `PlayFromStart` :!label _label)
      (:`Update`
        (`SceneComponent.K2_SetRelativeRotation` (`self.LeverPivot`) (`KismetMathLibrary.MakeRotator` _newtrack_1) false false))
      (:`Finished`
        (bind _returnvalue (`GameplayStatics.GetActorOfClass` "/Game/Content/Blueprints/Interraction/BP_DropLever.BP_DropLever_C"))
        (`/Game/Content/Blueprints/Interraction/BP_DropLever.Reload` _returnvalue)
        (if (`/Game/Content/Blueprints/Interraction/BP_ChandeliarTrap.Down` (`self.Chandeliar`))
          (set `/Game/Content/Blueprints/Interraction/BP_Interractable.CanBeInterracted` false (`self.As BP Interractable`)))))))

(event `BB`
  (if (`/Game/Content/Blueprints/Interraction/BP_ChandeliarTrap.Down` (`self.Chandeliar`))
    (`/Game/Content/Blueprints/Interraction/BP_ChandeliarTrap.StopArming` (`self.Chandeliar`))
    (goto _label :!via `Reverse`)))

(event `Reload`
  (`SceneComponent.K2_SetRelativeRotation` (`self.LeverPivot`) (`KismetMathLibrary.MakeRotator` -50.0) false false)
  (set `/Game/Content/Blueprints/Interraction/BP_Interractable.CanBeInterracted` true (`self.As BP Interractable`)))

(fn `UserConstructionScript`)