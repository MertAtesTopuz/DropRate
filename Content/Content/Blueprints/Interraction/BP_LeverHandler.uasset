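; BP_LeverHandler is a pickup for a lever handle that the player collects to equip a lever elsewhere in the level.
; On BeginPlay it registers itself with its BP_Interractable child actor and binds to that actor's interaction result.
; GainHandle flags the referenced Lever as having its handle, shows a message on the first-person character's UI, plays a sound, hides itself and is destroyed after a short delay.
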(event `self.ReceiveBeginPlay`
  (bind _asbp_interractable (cast `/Game/Content/Blueprints/Interraction/BP_Interractable` (`ChildActorComponent.ChildActor` (`self.ChildActor`))))
  (set `/Game/Content/Blueprints/Interraction/BP_Interractable.InterractionObject` self _asbp_interractable)
  (add `/Game/Content/Blueprints/Interraction/BP_Interractable.InterractionResult` _asbp_interractable (`|CreateDelegate` :!event `GainHandle`)))

(event `GainHandle`
  (params (Result :type Boolean))
  (bind _lever (`self.Lever`)
    (:`then`
      (set `/Game/Content/Blueprints/Interraction/BP_HandleMissingLever.HasLever` true _lever)
      (bind _returnvalue (`GameplayStatics.GetActorOfClass` "/Game/Content/Blueprints/Player/BP_FirstPersonCharacter.BP_FirstPersonCharacter_C"))
      (`/Game/Content/Blueprints/UI/WBP_MainUI.UIInfoText` (`/Game/Content/Blueprints/Player/BP_FirstPersonCharacter.UI` _returnvalue) "Hanndle Acquired")
      (`ActorComponent.K2_DestroyComponent` (`self.ChildActor`))
      (`GameplayStatics.SpawnSound2D` "/Game/Content/SFXsSenior/QuestItemGrab_Cue.QuestItemGrab_Cue" 1.0 1.0 0.0 null)
      (`self.SetActorHiddenInGame` true)
      (`KismetSystemLibrary.Delay` 2.0)
      (`self.K2_DestroyActor`))
    (:`else`)))

(fn `UserConstructionScript`)