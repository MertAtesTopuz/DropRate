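; Lever socket actor that requires a missing lever to be placed before it can operate a linked door.
; A child BP_Interractable reports interactions back, showing "Lever Missing" until HasLever is set externally.
; The first valid interaction reveals the lever mesh and changes the interaction type and widget.
; Later ones play a sound and flip-flop a timeline that rotates the pivot, calling OpenCloseDoor when finished.
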(event `self.ReceiveBeginPlay`
  (`|ExecutionSequence`
    (:`then_0`
      (bind _asbp_first_person_character (cast `/Game/Content/Blueprints/Player/BP_FirstPersonCharacter` (`GameplayStatics.GetPlayerCharacter` 0)))
      (set `self.Player` _asbp_first_person_character))
    (:`then_1`
      (bind _asbp_interractable (cast `/Game/Content/Blueprints/Interraction/BP_Interractable` (`ChildActorComponent.ChildActor` (`self.ChildActor`))))
      (set `/Game/Content/Blueprints/Interraction/BP_Interractable.InterractionObject` self _asbp_interractable)
      (add `/Game/Content/Blueprints/Interraction/BP_Interractable.InterractionResult` _asbp_interractable (`|CreateDelegate` :!event `SwitchLever`)))))

(event `SwitchLever`
  (params (Reasult :type Boolean))
  (bind _asbp_interractable (cast `/Game/Content/Blueprints/Interraction/BP_Interractable` (`ChildActorComponent.ChildActor` (`self.ChildActor`)) :!pure true))
  (if (`self.HasLever`)
    (if (`self.LeverPlaced`)
      (`GameplayStatics.SpawnSound2D` "/Game/Content/Assets/Sounds/SoundWaves/SW_Lever.SW_Lever" 1.0 1.0 0.0 null)
      (`/Engine/EditorBlueprintResources/StandardMacros.FlipFlop`
        (:`A`
          (bind (_direction _newtrack_1) (`Timeline|UseLeverTimeline` :!via `PlayFromStart` :!label _label)
            (:`Update`
              (`SceneComponent.K2_SetRelativeRotation` (`self.LeverPivot`) (`KismetMathLibrary.MakeRotator` _newtrack_1) false false))
            (:`Finished`
              (`/Game/Content/Blueprints/Interraction/BP_Door.Open/CloseDoor` (`self.Door`) true))))
        (:`B`
          (goto _label :!via `Reverse`)))
      (else
        (bind _returnvalue (`GameplayStatics.GetActorOfClass` "/Game/Content/Blueprints/Player/BP_FirstPersonCharacter.BP_FirstPersonCharacter_C"))
        (`/Game/Content/Blueprints/UI/WBP_MainUI.UIInfoText` (`/Game/Content/Blueprints/Player/BP_FirstPersonCharacter.UI` _returnvalue) "Lever Placed")
        (set `self.LeverPlaced` true)
        (`SceneComponent.SetVisibility` (`self.LockSlide`) true false)
        (set `/Game/Content/Blueprints/Interraction/BP_Interractable.InterractionType` "NewEnumerator2" _asbp_interractable)
        (set `/Game/Content/Blueprints/Interraction/BP_Interractable.ShouldWidgetHide` true _asbp_interractable)
        (`Widget.SetVisibility` (`/Game/Content/Blueprints/UI/WBP_F.F_Cog` (`/Game/Content/Blueprints/Interraction/BP_Interractable.InterractWidget` _asbp_interractable)) "Visible")))
    (else
      (bind _returnvalue_2 (`GameplayStatics.GetActorOfClass` "/Game/Content/Blueprints/Player/BP_FirstPersonCharacter.BP_FirstPersonCharacter_C"))
      (`/Game/Content/Blueprints/UI/WBP_MainUI.UIInfoText` (`/Game/Content/Blueprints/Player/BP_FirstPersonCharacter.UI` _returnvalue_2) "Lever Missing"))))

(fn `UserConstructionScript`)