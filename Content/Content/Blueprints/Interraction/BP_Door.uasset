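; BP_Door is a door actor that swings open and closed, either through its own interactable child actor or as a lever door.
; On BeginPlay a lever door destroys that child; otherwise the door registers itself with the BP_Interractable child and binds to its interaction result.
; Open/CloseDoor flip-flops a timeline driving door yaw, playing an unlock sound only on the forward swing and toggling IsOpen when the timeline finishes.
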(event `self.ReceiveBeginPlay`
  (if (`self.isLeverDoor`)
    (`ActorComponent.K2_DestroyComponent` (`self.ChildActor`))
    (else
      (bind _asbp_interractable (cast `/Game/Content/Blueprints/Interraction/BP_Interractable` (`ChildActorComponent.ChildActor` (`self.ChildActor`))))
      (set `/Game/Content/Blueprints/Interraction/BP_Interractable.InterractionObject` self _asbp_interractable)
      (add `/Game/Content/Blueprints/Interraction/BP_Interractable.InterractionResult` _asbp_interractable (`|CreateDelegate` :!event `Open/CloseDoor`)))))

(event `Open/CloseDoor`
  (params (Result :type Boolean))
  (`/Engine/EditorBlueprintResources/StandardMacros.FlipFlop`
    (:`A`
      (`GameplayStatics.PlaySound2D` "/Game/Content/Assets/Sounds/SoundWaves/SW_UnlockWoodenDoor.SW_UnlockWoodenDoor" 1.0 1.0 0.0 null null)
      (bind (_direction _newtrack_0) (`Timeline|Open/CloseAnim` :!via `PlayFromStart` :!label _label)
        (:`Update`
          (`SceneComponent.K2_SetRelativeRotation` (`self.Door`) (`KismetMathLibrary.MakeRotator` 0.0 0.0 _newtrack_0) false false))
        (:`Finished`
          (set `self.isOpen` (not (`self.isOpen`))))))
    (:`B`
      (goto _label :!via `Reverse`))))

(fn `UserConstructionScript`)