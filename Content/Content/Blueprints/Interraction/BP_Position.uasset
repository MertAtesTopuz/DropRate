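; BP_Position is an actor that travels in a loop along the spline of a BP_DanceSpline found at BeginPlay.
; ChangeState starts or clears a fast looping timer and is switched on immediately at start.
; WalkingTimerFunction finds the actor's current distance on the spline, advances one unit, wraps to zero past the end and applies that location and rotation.
; Movement speed therefore follows the timer rate rather than delta time.
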(event `self.ReceiveBeginPlay`
  (bind _returnvalue (`GameplayStatics.GetActorOfClass` "/Game/Content/Blueprints/Interraction/BP_DanceSpline.BP_DanceSpline_C"))
  (set `self.DanceRoute` _returnvalue)
  (`self.ChangeState` true))

(fn `ChangeState`
  (params (Walking :type Boolean))
  (set `self.Walking` Walking)
  (if (`local.Walking`)
    (bind _returnvalue (`KismetSystemLibrary.K2_SetTimerDelegate` (`|CreateDelegate` :!event `WalkingTimerFunction`) 0.01 true false -1.0))
    (set `self.WalkTimer` _returnvalue)
    (else
      (`KismetSystemLibrary.K2_ClearAndInvalidateTimerHandle` (`self.WalkTimer`)))))

(fn `UserConstructionScript`)

(fn `WalkingTimerFunction`
  (bind _spline (`/Game/Content/Blueprints/Interraction/BP_DanceSpline.Spline` (`self.DanceRoute`)))
  (bind _returnvalue (+ (`SplineComponent.GetDistanceAlongSplineAtLocation` _spline (`self.K2_GetActorLocation`) "World") 1.0))
  (bind (_returnvalue_location _returnvalue_rotation) (`KismetMathLibrary.BreakTransform` (`SplineComponent.GetTransformAtDistanceAlongSpline` _spline (select `bool` (> _returnvalue (`SplineComponent.GetSplineLength` _spline)) :`false` _returnvalue) "World" false)))
  (`self.K2_SetActorLocationAndRotation` _returnvalue_location _returnvalue_rotation))