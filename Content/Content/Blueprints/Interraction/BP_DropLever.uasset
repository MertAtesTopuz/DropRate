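; BP_DropLever is an interactable lever that drops the level's chandelier trap.
; It finds BP_ChandeliarTrap at BeginPlay and binds to the interaction result of its child BP_Interractable.
; Switching plays a sound and, if the chandelier is up, drops it, disables interaction and animates the pivot via timeline, then calls Reload on BP_ArmLever.
; Its own Reload resets the pivot and re-enables interaction.
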(event `self.ReceiveBeginPlay`
  (`|ExecutionSequence`
    (:`then_0`
      (bind _asbp_first_person_character (cast `/Game/Content/Blueprints/Player/BP_FirstPersonCharacter` (`GameplayStatics.GetPlayerCharacter` 0)))
      (set `self.Player` _asbp_first_person_character)
      (bind _returnvalue (`GameplayStatics.GetActorOfClass` "/Game/Content/Blueprints/Interraction/BP_ChandeliarTrap.BP_ChandeliarTrap_C"))
      (set `self.Chandeliar` _returnvalue))
    (:`then_1`
      (bind _asbp_interractable (cast `/Game/Content/Blueprints/Interraction/BP_Interractable` (`ChildActorComponent.ChildActor` (`self.ChildActor`))))
      (set `self.As BP Interractable` _asbp_interractable)
      (set `/Game/Content/Blueprints/Interraction/BP_Interractable.InterractionObject` self _asbp_interractable)
      (add `/Game/Content/Blueprints/Interraction/BP_Interractable.InterractionResult` _asbp_interractable (`|CreateDelegate` :!event `SwitchLever`)))))

(event `SwitchLever`
  (params (Reasult :type Boolean))
  (bind _chandeliar (`self.Chandeliar`))
  (`GameplayStatics.SpawnSound2D` "/Game/Content/Assets/Sounds/SoundWaves/SW_Lever.SW_Lever" 1.0 1.0 0.0 null)
  (if (not (`/Game/Content/Blueprints/Interraction/BP_ChandeliarTrap.Down` _chandeliar))
    (`/Game/Content/Blueprints/Interraction/BP_ChandeliarTrap.GoDown` _chandeliar)
    (set `/Game/Content/Blueprints/Interraction/BP_Interractable.CanBeInterracted` false (`self.As BP Interractable`))
    (bind (_direction _newtrack_1) (`Timeline|UseLeverTimeline` :!via `PlayFromStart`)
      (:`Update`
        (`SceneComponent.K2_SetRelativeRotation` (`self.LeverPivot`) (`KismetMathLibrary.MakeRotator` _newtrack_1) false false))
      (:`Finished`
        (bind _returnvalue (`GameplayStatics.GetActorOfClass` "/Game/Content/Blueprints/Interraction/BP_ArmLever.BP_ArmLever_C"))
        (`/Game/Content/Blueprints/Interraction/BP_ArmLever.Reload` _returnvalue)))))

(event `Reload`
  (`SceneComponent.K2_SetRelativeRotation` (`self.LeverPivot`) (`KismetMathLibrary.MakeRotator` -50.0) false false)
  (set `/Game/Content/Blueprints/Interraction/BP_Interractable.CanBeInterracted` true (`self.As BP Interractable`)))

(fn `UserConstructionScript`)