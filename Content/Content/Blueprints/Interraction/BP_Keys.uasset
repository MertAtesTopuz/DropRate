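; BP_Keys is a pickup key that unlocks an assigned Door when the player interacts with it.
; On BeginPlay it registers itself with its child BP_Interractable actor and binds to that interaction result.
; GainKey flags the Door as having a key, shows "Key Acquired" on the first-person character's UI, plays a grab sound, removes the interactable, then hides and destroys itself after a delay.
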(event `self.ReceiveBeginPlay`
  (bind _asbp_interractable (cast `/Game/Content/Blueprints/Interraction/BP_Interractable` (`ChildActorComponent.ChildActor` (`self.ChildActor`))))
  (set `/Game/Content/Blueprints/Interraction/BP_Interractable.InterractionObject` self _asbp_interractable)
  (add `/Game/Content/Blueprints/Interraction/BP_Interractable.InterractionResult` _asbp_interractable (`|CreateDelegate` :!event `GainKey`)))

(event `GainKey`
  (params (Result :type Boolean))
  (bind _door (`self.Door`)
    (:`then`
      (set `/Game/Content/Blueprints/Interraction/BP_KeyLockedDoor.HasKey` true _door)
      (bind _returnvalue (`GameplayStatics.GetActorOfClass` "/Game/Content/Blueprints/Player/BP_FirstPersonCharacter.BP_FirstPersonCharacter_C"))
      (`/Game/Content/Blueprints/UI/WBP_MainUI.UIInfoText` (`/Game/Content/Blueprints/Player/BP_FirstPersonCharacter.UI` _returnvalue) "Key Acquired")
      (`ActorComponent.K2_DestroyComponent` (`self.ChildActor`))
      (`GameplayStatics.SpawnSound2D` "/Game/Content/Assets/Sounds/SoundWaves/SW_Grabbing_Key.SW_Grabbing_Key" 1.0 1.0 0.0 null)
      (`self.SetActorHiddenInGame` true)
      (`KismetSystemLibrary.Delay` 2.0)
      (`self.K2_DestroyActor`))
    (:`else`)))

(fn `UserConstructionScript`)