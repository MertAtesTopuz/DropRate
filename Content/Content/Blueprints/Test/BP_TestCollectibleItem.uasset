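; Test collectible item actor that the first-person player can pick up into their inventory.
; A child BP_Interractable, with a configurable box extent, reports interaction results back, while IsInterractionSuccessful checks inventory space.
; Success adds ItemData to the player and destroys the actor if accepted; failure plays the inventory-full UI animation.
; Both outcomes play a grab sound chosen by matching the item's mesh.
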(event `self.ReceiveBeginPlay`
  (`|ExecutionSequence`
    (:`then_0`
      (bind _asbp_first_person_character (cast `/Game/Content/Blueprints/Player/BP_FirstPersonCharacter` (`GameplayStatics.GetPlayerCharacter` 0)))
      (set `self.Player` _asbp_first_person_character))
    (:`then_1`
      (bind _asbp_interractable (cast `/Game/Content/Blueprints/Interraction/BP_Interractable` (`ChildActorComponent.ChildActor` (`self.ChildActor`))))
      (set `/Game/Content/Blueprints/Interraction/BP_Interractable.InterractionObject` self _asbp_interractable)
      (add `/Game/Content/Blueprints/Interraction/BP_Interractable.InterractionResult` _asbp_interractable (`|CreateDelegate` :!event `CollectItem`)))))

(event `CollectItem`
  (params (Result :type Boolean))
  (bind _item_data (`self.Item Data`))
  (if Result
    (bind _newparam (`self.SoundChooser` _item_data))
    (`GameplayStatics.SpawnSound2D` _newparam 1.0 1.0 0.0 null)
    (bind _returnvalue (`/Game/Content/Blueprints/Player/BP_FirstPersonCharacter.CollectItem` (`self.Player`) (`self.Item Data`)))
    (if _returnvalue
      (`self.K2_DestroyActor`))
    (else
      (bind _newparam_2 (`self.SoundChooser` _item_data))
      (`GameplayStatics.SpawnSound2D` _newparam_2 1.0 1.0 0.0 null)
      (`/Game/Content/Blueprints/UI/WBP_MainUI.PlayInventoryFullAnimation` (`/Game/Content/Blueprints/Player/BP_FirstPersonCharacter.UI` (`self.Player`))))))

(fn `IsInterractionSuccessful`
  (returns (ReturnValue :type Boolean))
  (bind _asbp_first_person_character (cast `/Game/Content/Blueprints/Player/BP_FirstPersonCharacter` (`GameplayStatics.GetPlayerCharacter` 0)))
  (return (<= (`KismetArrayLibrary.Array_Length` (`/Game/Content/Blueprints/Player/BP_FirstPersonCharacter.Inventory` _asbp_first_person_character)) 3)))

(fn `SoundChooser`
  (params (Data :type "/Game/Content/Blueprints/Data/ST_ItemData Structure"))
  (returns (NewParam :type "SoundBase Object Reference"))
  (bind (_name _mesh) (break `/Game/Content/Blueprints/Data/ST_ItemData` Data))
  (if (== _mesh "/Game/Content/Assets/Meshes/Doll_MonsterHeadBroken.Doll_MonsterHeadBroken")
    (return "/Game/Content/SFXsSenior/MetalHeadGrab_Cue.MetalHeadGrab_Cue")
    (elif (== _mesh "/Game/Content/Assets/Meshes/SM_HandheldBat.SM_HandheldBat")
      (return "/Game/Content/SFXsSenior/BaseballBatGrab_Cue.BaseballBatGrab_Cue")
      (elif (== _mesh "/Game/Content/Assets/Meshes/SM_Throwing_Bottle.SM_Throwing_Bottle")
        (return "/Game/Content/SFXsSenior/CamSiseGrab_Cue.CamSiseGrab_Cue")
        (else
          (return "/Game/Content/SFXsSenior/Grab4_Cue.Grab4_Cue"))))))

(fn `UserConstructionScript`
  (`StaticMeshComponent.SetStaticMesh` (`self.Sphere`) (`self.ItemMesh`))
  (`BoxComponent.SetBoxExtent` (`/Game/Content/Blueprints/Interraction/BP_Interractable.Box` (cast `/Game/Content/Blueprints/Interraction/BP_Interractable` (`ChildActorComponent.ChildActor` (`self.ChildActor`)) :!pure true)) (`self.Box Extend`) true))