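; Test jumpscare actor that triggers when the player character overlaps its Box.
; It blends the camera to its own view, then plays its Mesh animation once while disabling player input and hiding the character.
; After a fixed delay it restores input and visibility and blends the view back to the player.
; The sequence is driven by Delays, with no guard against retriggering.
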(event `self.Box.OnComponentBeginOverlap`
  (params (OverlappedComponent :type "PrimitiveComponent Object Reference") (OtherActor :type "Actor Object Reference") (OtherComp :type "PrimitiveComponent Object Reference") (OtherBodyIndex :type Integer) (bFromSweep :type Boolean) (SweepResult :type "HitResult Structure (by ref)"))
  (bind _returnvalue (`GameplayStatics.GetPlayerCharacter` 0))
  (bind _returnvalue_2 (`GameplayStatics.GetPlayerCharacter` 0))
  (if (== OtherActor (`GameplayStatics.GetPlayerCharacter` 0))
    (`PlayerController.SetViewTargetWithBlend` (`GameplayStatics.GetPlayerController` 0) self 0.5 "VTBlend_Linear" 0.0 false)
    (`KismetSystemLibrary.Delay` 0.5)
    (`SkeletalMeshComponent.Play` (`self.Mesh`) false)
    (`self.DisableInput` _returnvalue (`GameplayStatics.GetPlayerController` 0))
    (`self.SetActorHiddenInGame` _returnvalue true)
    (`KismetSystemLibrary.Delay` 6.0)
    (`self.EnableInput` _returnvalue_2 (`GameplayStatics.GetPlayerController` 0))
    (`self.SetActorHiddenInGame` _returnvalue_2 false)
    (`PlayerController.SetViewTargetWithBlend` (`GameplayStatics.GetPlayerController` 0) (`GameplayStatics.GetPlayerCharacter` 0) 0.3 "VTBlend_Linear" 0.0 false)))

(fn `UserConstructionScript`)