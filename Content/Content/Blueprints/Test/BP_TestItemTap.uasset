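; BP_TestItemTap is a test interactable item that opens an inspect UI when an interaction succeeds.
; On BeginPlay it registers itself as the interaction object on its BP_Interractable child actor and binds a result event.
; Its success check always returns true, and a successful result plays a document-grab sound and adds WBP_InspectUI to the viewport.
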(event `self.ReceiveBeginPlay`
  (bind _asbp_interractable (cast `/Game/Content/Blueprints/Interraction/BP_Interractable` (`ChildActorComponent.ChildActor` (`self.ChildActor`))))
  (set `/Game/Content/Blueprints/Interraction/BP_Interractable.InterractionObject` self _asbp_interractable)
  (add `/Game/Content/Blueprints/Interraction/BP_Interractable.InterractionResult` _asbp_interractable (`|CreateDelegate` :!event `CreateInspectUI`)))

(event `CreateInspectUI`
  (params (Result :type Boolean))
  (if Result
    (`GameplayStatics.SpawnSound2D` "/Game/Content/Assets/Sounds/SoundWaves/SW_DocumentGrabbing.SW_DocumentGrabbing" 1.0 1.0 0.0 null)
    (bind _returnvalue (`|CreateWidget` "/Game/Content/Blueprints/UI/WBP_InspectUI.WBP_InspectUI_C" (`GameplayStatics.GetPlayerController` 0)))
    (`UserWidget.AddToViewport` _returnvalue 0)))

(fn `IsInterractionSuccessful`
  (returns (ReturnValue :type Boolean))
  (return true))

(fn `UserConstructionScript`)