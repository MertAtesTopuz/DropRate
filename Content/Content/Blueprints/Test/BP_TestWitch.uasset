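; Test witch AI pawn that walks up to and executes either a selected enemy or the player.
; Start runs a timed sequence toggling the enemy's state, then kills it, using montage notifies to swap it for a hand-held mesh, drop a ragdoll and walk back.
; KillPlayer hides and disables the player, blending the view to the witch's camera.
; Tick pins that mesh, and conditionally the camera, to the left-hand socket.
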(event `KillPlayer`
  (bind _returnvalue (`GameplayStatics.GetPlayerCharacter` 0))
  (`|AIMoveTo` self (0.0 0.0 0.0) _returnvalue 10.0
    (:`OnSuccess`
      (`self.SetActorHiddenInGame` _returnvalue true)
      (`self.DisableInput` (`GameplayStatics.GetPlayerCharacter` 0) (`GameplayStatics.GetPlayerController` 0))
      (`|ExecutionSequence`
        (:`then_0`
          (`KismetSystemLibrary.Delay` 0.2)
          (`PlayerController.SetViewTargetWithBlend` (`GameplayStatics.GetPlayerController` 0) self 0.2 "VTBlend_Linear" 0.0 false))
        (:`then_1`
          (`|PlayMontage` (`self.Mesh`) "/Game/Content/Assets/Animations/AnimationSequences/AM_Execute.AM_Execute" 0.5
            (:`OnNotifyBegin`
              (`/Engine/EditorBlueprintResources/StandardMacros.FlipFlop`
                (:`A`
                  (set `self.Condition` true))
                (:`B`
                  (bind (_direction _newtrack_0) (`Timeline|Timeline` :!via `PlayFromStart`)
                    (:`Update`
                      (`SceneComponent.K2_SetRelativeRotation` (`self.Camera`) (`KismetMathLibrary.MakeRotator` _newtrack_0 0.0 -180.0) false false))))))))))))

(event `Start`
  (`KismetSystemLibrary.Delay` 12.1)
  (`/Game/Content/Blueprints/Interraction/BP_DanceEnemy.ChangeState` (`self.Enemy`) true)
  (`KismetSystemLibrary.Delay` 1.0)
  (`/Game/Content/Blueprints/Interraction/BP_DanceEnemy.ChangeState` (`self.Enemy`) false)
  (`KismetSystemLibrary.Delay` 1.0)
  (`self.KillSelectedEnemy`)
  (set `self.NewVar` (`self.K2_GetActorLocation`)))

(event `self.ReceiveTick`
  (params (DeltaSeconds :type "Float (single-precision)"))
  (`|ExecutionSequence`
    (:`then_0`
      (if (`self.Condition`)
        (`SceneComponent.K2_SetWorldLocation` (`self.Camera`) (+ (`SceneComponent.GetSocketLocation` (`self.Mesh`) "Hand_L") (0.0 0.0 12.0) (* (`SceneComponent.GetForwardVector` (`self.Camera`)) -11.0)) false false)))
    (:`then_1`
      (`SceneComponent.K2_SetWorldLocation` (`self.SkeletalMesh`) (+ (`SceneComponent.GetSocketLocation` (`self.Mesh`) "Hand_L") (0.0 0.0 -110.0)) false false))))

(event `KillSelectedEnemy`
  (`|AIMoveTo` self (0.0 0.0 0.0) (`self.Enemy`) 60.0 true
    (:`OnSuccess`
      (`|PlayMontage` (`self.Mesh`) "/Game/Content/Assets/Animations/AnimationSequences/AM_Execute.AM_Execute" 0.5
        (:`OnNotifyBegin`
          (`/Engine/EditorBlueprintResources/StandardMacros.FlipFlop`
            (:`A`
              (`SceneComponent.SetVisibility` (`self.SkeletalMesh`) true false)
              (bind _enemy (`self.Enemy`)
                (:`then`
                  (`self.K2_DestroyActor` _enemy))
                (:`else`)))
            (:`B`
              (`|SpawnActorFromClass` "/Game/Content/Blueprints/Interraction/BP_Ragdoll.BP_Ragdoll_C" (`KismetMathLibrary.MakeTransform` (`SceneComponent.GetSocketLocation` (`self.Mesh`) "Hand_L") (struct :`Pitch` 11.0 :`Yaw` 90.0)) "Undefined" "MultiplyWithRoot" null null)
              (`SceneComponent.SetVisibility` (`self.SkeletalMesh`) false false)
              (`self.StopAnimMontage` (`self.GetCurrentMontage`))
              (`KismetSystemLibrary.Delay` 2.0)
              (`|AIMoveTo` self (`self.NewVar`) null 10.0))))))))

(fn `UserConstructionScript`)