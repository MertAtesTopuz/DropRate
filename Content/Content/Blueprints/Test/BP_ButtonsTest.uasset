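; BP_ButtonsTest is a test actor that drives three staged buttons from child BP_Interractable actors.
; On BeginPlay it binds each child's interaction result to its own event, which passes that button's index to InterractWithButton.
; That function selects the button's state counter and mesh by index: the first press only advances the state, the second unhides the mesh and advances again, and later presses print the mesh's name.
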(event `self.ReceiveBeginPlay`
  (add `/Game/Content/Blueprints/Interraction/BP_Interractable.InterractionResult` (cast `/Game/Content/Blueprints/Interraction/BP_Interractable` (`ChildActorComponent.ChildActor` (`self.ChildActor0`)) :!pure true) (`|CreateDelegate` :!event `ButtonPressed1`))
  (add `/Game/Content/Blueprints/Interraction/BP_Interractable.InterractionResult` (cast `/Game/Content/Blueprints/Interraction/BP_Interractable` (`ChildActorComponent.ChildActor` (`self.ChildActor1`)) :!pure true) (`|CreateDelegate` :!event `ButtonPressed2`))
  (add `/Game/Content/Blueprints/Interraction/BP_Interractable.InterractionResult` (cast `/Game/Content/Blueprints/Interraction/BP_Interractable` (`ChildActorComponent.ChildActor` (`self.ChildActor2`)) :!pure true) (`|CreateDelegate` :!event `ButtonPressed3`)))

(event `ButtonPressed1`
  (params (Value :type Boolean))
  (`self.InterractWithButton` 0))

(event `ButtonPressed2`
  (params (Value :type Boolean))
  (`self.InterractWithButton` 1))

(event `ButtonPressed3`
  (params (Value :type Boolean))
  (`self.InterractWithButton` 2))

(fn `InterractWithButton`
  (params (ButtonIndex :type Integer))
  (bind _returnvalue (select `int` (`local.ButtonIndex`) :`0` (`self.SM_Button0`) :`1` (`self.SM_Button1`) :`2` (`self.SM_Button2`) :!type "SceneComponent Object Reference"))
  (bind _returnvalue_2 (select `int` (`local.ButtonIndex`) :`0` (`self.ButtonState0`) :`1` (`self.ButtonState1`) :`2` (`self.ButtonState2`)))
  (switch `int` _returnvalue_2
    (:`0`
      (`/Engine/EditorBlueprintResources/StandardMacros.IncrementInt` _returnvalue_2))
    (:`1`
      (`SceneComponent.SetHiddenInGame` _returnvalue false false)
      (`/Engine/EditorBlueprintResources/StandardMacros.IncrementInt` _returnvalue_2))
    (:`2`
      (`KismetSystemLibrary.PrintString` (`KismetSystemLibrary.GetDisplayName` _returnvalue)))))

(fn `UserConstructionScript`)