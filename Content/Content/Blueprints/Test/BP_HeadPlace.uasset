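; BP_HeadPlace is an interaction spot where the player places an accepted key item, apparently a metal head.
; Hand updates show or clear a material preview when the selected item's mesh is in PlacableItems.
; Placing locks the preview through gates and, if Replacable, enables a child BP_Interractable for pickup.
; Pickup checks inventory space, maps the mesh to ItemDatas by index and resets the spot, or plays the inventory-full animation.
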(event `self.ReceiveBeginPlay`
  (bind _asbp_first_person_character (cast `/Game/Content/Blueprints/Player/BP_FirstPersonCharacter` (`GameplayStatics.GetPlayerCharacter` 0)))
  (bind _output_get (set `self.Player` _asbp_first_person_character))
  (add `/Game/Content/Blueprints/Player/BP_FirstPersonCharacter.UpdateHand` _output_get (`|CreateDelegate` :!event `HandUpdated`))
  (bind _asbp_interractable (cast `/Game/Content/Blueprints/Interraction/BP_Interractable` (`ChildActorComponent.ChildActor` (`self.ChildActor`))))
  (bind _output_get_2 (set `self.As BP Interractable` _asbp_interractable))
  (`self.SetActorEnableCollision` _output_get_2 false)
  (add `/Game/Content/Blueprints/Interraction/BP_Interractable.InterractionResult` _asbp_interractable (`|CreateDelegate` :!event `TryCollectinPlacedItem`)))

(event `HandUpdated`
  (if (`self.PlayerHasKeyItem`)
    (`/Game/Content/Blueprints/Management/BPI_Interract.ShowInterraction`)
    (else
      (`/Game/Content/Blueprints/Management/BPI_Interract.HideInterraction`))))

(event `/Game/Content/Blueprints/Management/BPI_Interract.ShowInterraction`
  (bind _sm_keyitem (`self.SM_KeyItem`))
  (`/Engine/EditorBlueprintResources/StandardMacros.Gate` false :!label _label
    (:`Exit`
      (if (`self.PlayerHasKeyItem`)
        (`StaticMeshComponent.SetStaticMesh` _sm_keyitem (`self.CurrentKeyItem`))
        (`PrimitiveComponent.SetMaterial` _sm_keyitem 0 "/Game/Content/Assets/Materials/M_ItemPreview.M_ItemPreview")))))

(event `/Game/Content/Blueprints/Management/BPI_Interract.HideInterraction`
  (`/Engine/EditorBlueprintResources/StandardMacros.Gate` false :!label _label_2
    (:`Exit`
      (`StaticMeshComponent.SetStaticMesh` (`self.SM_KeyItem`) null))))

(event `/Game/Content/Blueprints/Management/BPI_Interract.PressInterract`
  (`/Engine/EditorBlueprintResources/StandardMacros.DoOnce` false :!label _label_3
    (:`Completed`
      (`|ExecutionSequence`
        (:`then_0`
          (goto _label_2 :!via `Close`))
        (:`then_1`
          (goto _label :!via `Close`))
        (:`then_2`
          (`PrimitiveComponent.SetMaterial` (`self.SM_KeyItem`) 0 "/Game/Content/Assets/Materials/Doll_Monster/M_DollMon1_Metal_Head.M_DollMon1_Metal_Head")
          (if (`self.Replacable`)
            (`self.SetActorEnableCollision` (`self.As BP Interractable`) true)
            (set `self.isPlaced` true)
            (`GameplayStatics.PlaySound2D` "/Game/Content/SFXsSenior/MetalKafaYerlestir_Cue.MetalKafaYerlestir_Cue" 1.0 1.0 0.0 null null)))))))

(event `TryCollectinPlacedItem`
  (params (Result :type Boolean))
  (bind _asbp_first_person_character (cast `/Game/Content/Blueprints/Player/BP_FirstPersonCharacter` (`GameplayStatics.GetPlayerCharacter` 0)))
  (if (<= (`KismetArrayLibrary.Array_Length` (`/Game/Content/Blueprints/Player/BP_FirstPersonCharacter.Inventory` _asbp_first_person_character)) 3)
    (`|ExecutionSequence`
      (:`then_0`
        (goto _label :!via `Open`))
      (:`then_1`
        (goto _label_2 :!via `Open`))
      (:`then_2`
        (goto _label_3 :!via `Reset`))
      (:`then_3`
        (`GameplayStatics.SpawnSound2D` "/Game/Content/SFXsSenior/Grab4_Cue.Grab4_Cue" 1.0 1.0 0.0 null)
        (`/Game/Content/Blueprints/Player/BP_FirstPersonCharacter.CollectItem` (`self.Player`) (`|GetArrayItem` (`self.Item Datas`) (`KismetArrayLibrary.Array_Find` (`self.PlacableItems`) (`StaticMeshComponent.StaticMesh` (`self.SM_KeyItem`)))))
        (`self.SetActorEnableCollision` (`self.As BP Interractable`) false)
        (`StaticMeshComponent.SetStaticMesh` (`self.SM_KeyItem`) null)
        (set `self.isPlaced` false)))
    (else
      (`GameplayStatics.SpawnSound2D` "/Game/Content/SFXsSenior/Grab4_Cue.Grab4_Cue" 1.0 1.0 0.0 null)
      (`/Game/Content/Blueprints/UI/WBP_MainUI.PlayInventoryFullAnimation` (`/Game/Content/Blueprints/Player/BP_FirstPersonCharacter.UI` (`self.Player`))))))

(fn `IsInterractionSuccessful`
  (returns (ReturnValue :type Boolean))
  (return (`self.PlayerHasKeyItem`)))

(fn `PlayerHasKeyItem`
  (returns (ReturnValue :type Boolean))
  (bind ((`Mesh_7_F7BDD69646A74E31BED417B1D1DC6DD5` _mesh)) (break `/Game/Content/Blueprints/Data/ST_ItemData` (`/Game/Content/Blueprints/Player/BP_FirstPersonCharacter.SelectedItem` (`self.Player`))))
  (set `self.CurrentKeyItem` _mesh)
  (return (and (`KismetArrayLibrary.Array_Contains` (`self.PlacableItems`) _mesh) (== (`/Game/Content/Blueprints/Player/BP_FirstPersonCharacter.Interractable` (`self.Player`)) self))))

(fn `UserConstructionScript`)