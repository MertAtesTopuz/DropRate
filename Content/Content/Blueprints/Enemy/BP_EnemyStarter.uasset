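; BP_EnemyStarter is a trigger actor that starts a set of enemies when the player character overlaps it.
; StartEnemies loops over the Enemies array, casting each entry to BP_EnemyAi or, failing that, BP_EnemyAi2.
; It sets the OnJumpscare key to false on each matched AI's Blackboard, leaving any resulting behavior to logic outside this Blueprint.
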(event `self.ReceiveActorBeginOverlap`
  (params (OtherActor :type "Actor Object Reference"))
  (if (== OtherActor (`GameplayStatics.GetPlayerCharacter` 0))
    (`self.StartEnemies`)))

(event `StartEnemies`
  (for _array_element (`self.Enemies`)
    (bind _asbp_enemy_ai (cast `/Game/Content/Blueprints/Enemy/BP_EnemyAi` _array_element)
      (:`then`
        (`BlackboardComponent.SetValueAsBool` (`AIBlueprintHelperLibrary.GetBlackboard` _asbp_enemy_ai) "OnJumpscare" false))
      (:`CastFailed`
        (bind _asbp_enemy_ai_2 (cast `/Game/Content/Blueprints/Enemy/BP_EnemyAi2` _array_element))
        (`BlackboardComponent.SetValueAsBool` (`AIBlueprintHelperLibrary.GetBlackboard` _asbp_enemy_ai_2) "OnJumpscare" false)))))

(fn `UserConstructionScript`)