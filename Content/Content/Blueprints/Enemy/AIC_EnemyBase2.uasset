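; AI controller for an enemy that runs the Enemy2 behavior tree and tracks Passive, Investigate and Attack states in the Blackboard.
; Two perception components, swapped for default and investigate modes, share one update handler, though stimulus lookups always query the default one.
; Heard sounds while Passive or Investigating set Investigate with a point of interest.
; Damage sensing triggers nothing, and the sight-to-attack handler is never called here.
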(event `self.ReceivePossess`
  (params (PossessedPawn :type "Pawn Object Reference"))
  (`self.RunBehaviorTree` "/Game/Content/Blueprints/Enemy/BehaviorTree/BT_Enemy2BaseTree.BT_Enemy2BaseTree")
  (`self.SetStateAsPassive`))

(event `self.DefeultPerception.OnPerceptionUpdated`
  (params (UpdatedActors :type "Array of Actor Object Reference (by ref)"))
  (for _array_element (stale `self.InvestigatePerception.OnPerceptionUpdated` UpdatedActors) :!label _label
    (`|ExecutionSequence`
      (:`then_0`
        (bind (_sensed _stimulus) (`self.CanSenseActor` _array_element "NewEnumerator2"))
        (if _sensed
          (`self.HandleSenseSound` (`.StimulusLocation` (break `AIStimulus` _stimulus)))))
      (:`then_1`
        (bind _sensed_2 (`self.CanSenseActor` null "NewEnumerator3"))
        (if _sensed_2
          _)))))

(event `self.InvestigatePerception.OnPerceptionUpdated`
  (params (UpdatedActors :type "Array of Actor Object Reference (by ref)"))
  (goto _label))

(event `SetDefeultPerception`
  (set `self.InvestigateState` "NewEnumerator0")
  (`ActorComponent.SetActive` (`self.InvestigatePerception`) false false)
  (`ActorComponent.SetActive` (`self.DefeultPerception`) true false))

(event `SetInvestigatePerception`
  (set `self.InvestigateState` "NewEnumerator1")
  (`ActorComponent.SetActive` (`self.DefeultPerception`) false false)
  (`ActorComponent.SetActive` (`self.InvestigatePerception`) true false))

(fn `CanSenseActor`
  (params (Actor :type "Actor Object Reference") (Sense :type "/Game/Content/Blueprints/Data/E_AISense Enum" :default "NewEnumerator0"))
  (returns (Sensed :type Boolean) (Stimulus :type "AIStimulus Structure"))
  (bind _info (`AIPerceptionComponent.GetActorsPerception` (`self.DefeultPerception`) Actor))
  (for _array_element (`.LastSensedStimuli` (break `ActorPerceptionBlueprintInfo` _info))
    (bind _returnvalue (`AIPerceptionSystem.GetSenseClassForStimulus` _array_element))
    (if (== _returnvalue (select `/Game/Content/Blueprints/Data/E_AISense` Sense :`NewEnumerator1` "/Script/AIModule.AISense_Sight" :`NewEnumerator2` "/Script/AIModule.AISense_Hearing" :`NewEnumerator3` "/Script/AIModule.AISense_Damage" :!type "Object Class Reference"))
      (return (`.bSuccessfullySensed` (break `AIStimulus` _array_element)) _array_element))))

(fn `GetCurrentState`
  (returns (State :type "/Game/Content/Blueprints/Data/E_EnemyStates Enum"))
  (return (cast `/Game/Content/Blueprints/Data/E_EnemyStates` (`BlackboardComponent.GetValueAsEnum` (`self.Blackboard`) (`self.StateKey`)))))

(fn `HandleSenseSight`
  (params (NewParam :type "Actor Object Reference"))
  (bind _state (`self.GetCurrentState`))
  (switch `/Game/Content/Blueprints/Data/E_EnemyStates` _state
    (:`NewEnumerator0`
      _)
    (:`NewEnumerator2`
      _))
  (if (== NewParam (`GameplayStatics.GetPlayerCharacter` 0))
    (`self.SetStateAsAttack` NewParam)))

(fn `HandleSenseSound`
  (params (Location :type "Vector Structure"))
  (bind _state (`self.GetCurrentState`))
  (switch `/Game/Content/Blueprints/Data/E_EnemyStates` _state
    (:`NewEnumerator0`
      _)
    (:`NewEnumerator2`
      _))
  (`self.SetStateAsInvestigate` Location))

(fn `SetInvestigateValue`)

(fn `SetStateAsAttack`
  (params (AttackTarget :type "Actor Object Reference"))
  (`BlackboardComponent.SetValueAsEnum` (`self.Blackboard`) (`self.StateKey`) (enumliteral `/Game/Content/Blueprints/Data/E_EnemyStates` "NewEnumerator1"))
  (`BlackboardComponent.SetValueAsObject` (`self.Blackboard`) (`self.AttackTargetKey`) (`GameplayStatics.GetPlayerCharacter` 0)))

(fn `SetStateAsInvestigate`
  (params (Location :type "Vector Structure"))
  (`BlackboardComponent.SetValueAsEnum` (`self.Blackboard`) (`self.StateKey`) (enumliteral `/Game/Content/Blueprints/Data/E_EnemyStates` "NewEnumerator2"))
  (`BlackboardComponent.SetValueAsVector` (`self.Blackboard`) (`self.PointOfInterestKeyName`) Location))

(fn `SetStateAsPassive`
  (`BlackboardComponent.SetValueAsEnum` (`self.Blackboard`) (`self.StateKey`) (enumliteral `/Game/Content/Blueprints/Data/E_EnemyStates` "NewEnumerator0")))

(fn `SetTargetVector`
  (params (TargetVector :type "Vector Structure"))
  (`BlackboardComponent.SetValueAsVector` (`self.Blackboard`) (`self.TargetVectorKey`) TargetVector))

(fn `UserConstructionScript`)