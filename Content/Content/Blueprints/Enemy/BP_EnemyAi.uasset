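; Doll monster enemy character that patrols and attacks the player, and leaves a collectible head when killed.
; Interface functions feed its blackboard and AI controller patrol, perception and speed settings.
; A looping-timer sphere trace on the right palm turns a successful hit into a camera-blend jumpscare that freezes time.
; Damage plays death montages and enables a child interactable, which adds the head to inventory and hides it via material parameter.
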(event `self.ReceiveBeginPlay`
  (`self.Start`)
  (bind _asbp_interractable (cast `/Game/Content/Blueprints/Interraction/BP_Interractable` (`ChildActorComponent.ChildActor` (`self.ChildActor`))))
  (add `/Game/Content/Blueprints/Interraction/BP_Interractable.InterractionResult` _asbp_interractable (delegate `RemoveHead`)))

(event `RemoveHead`
  (params (Result :type Boolean))
  (if (<= (`KismetArrayLibrary.Array_Length` (`/Game/Content/Blueprints/Player/BP_FirstPersonCharacter.Inventory` (cast `/Game/Content/Blueprints/Player/BP_FirstPersonCharacter` (`GameplayStatics.GetPlayerCharacter` 0) :!pure true))) 3)
    (`GameplayStatics.SpawnSound2D` "/Game/Content/Assets/Sounds/SoundWaves/SW_GrabItem.SW_GrabItem" 1.0 1.0 0.0 null)
    (bind _returnvalue (`/Game/Content/Blueprints/Player/BP_FirstPersonCharacter.CollectItem` (cast `/Game/Content/Blueprints/Player/BP_FirstPersonCharacter` (`GameplayStatics.GetPlayerCharacter` 0) :!pure true) (make `/Game/Content/Blueprints/Data/ST_ItemData` "Head" "/Game/Content/Assets/Meshes/Doll_Monster_Head.Doll_Monster_Head" "/Game/Content/Assets/Textures/Doll_Monster/doll_mon1_metal_head/T_doll_monster5_DefaultMaterial_AO.T_doll_monster5_DefaultMaterial_AO" "NewEnumerator5")))
    (if _returnvalue
      (bind _returnvalue_2 (`PrimitiveComponent.CreateDynamicMaterialInstance` (`self.Mesh`) 0 null "None"))
      (`MaterialInstanceDynamic.SetScalarParameterValue` _returnvalue_2 "HeadVisible" 0.0))
    (else
      (`GameplayStatics.SpawnSound2D` "/Game/Content/Assets/Sounds/SoundWaves/SW_GrabItem.SW_GrabItem" 1.0 1.0 0.0 null)
      (`/Game/Content/Blueprints/UI/WBP_MainUI.PlayInventoryFullAnimation` (`/Game/Content/Blueprints/Player/BP_FirstPersonCharacter.UI` (cast `/Game/Content/Blueprints/Player/BP_FirstPersonCharacter` (`GameplayStatics.GetPlayerCharacter` 0) :!pure true))))))

(event `Start`
  (`self.PatrolRoute`
    (:`then`
      (`KismetSystemLibrary.Delay` 0.2)
      (`BlackboardComponent.SetValueAsBool` (`AIBlueprintHelperLibrary.GetBlackboard` null) "HasPatrol" true))
    (:`else`)))

(event `TakeDamage`
  (`|ExecutionSequence`
    (:`then_0`
      (`BlackboardComponent.SetValueAsBool` (`AIBlueprintHelperLibrary.GetBlackboard` null) "OnJumpscare" true)
      (`|PlayMontage` (`self.Mesh`) "/Game/Content/Assets/Animations/AnimationMontages/doll_monster_damage_Montage.doll_monster_damage_Montage"
        (:`OnCompleted`
          (`|PlayMontage` (`self.Mesh`) "/Game/Content/Assets/Animations/AnimationMontages/doll_monster_death_Montage.doll_monster_death_Montage"
            (:`then`
              (`KismetSystemLibrary.Delay` 0.7)
              (set `/Game/Content/Blueprints/Interraction/BP_Interractable.CanBeInterracted` true (cast `/Game/Content/Blueprints/Interraction/BP_Interractable` (`ChildActorComponent.ChildActor` (`self.ChildActor`)) :!pure true)))))))
    (:`then_1`
      (`AIController.K2_ClearFocus` (`AIBlueprintHelperLibrary.GetAIController` self))
      (`self.SetActorEnableCollision` false))))

(event `JumpscareAnim`
  (`BlackboardComponent.SetValueAsBool` (`AIBlueprintHelperLibrary.GetBlackboard` null) "OnJumpscare" true)
  (`PlayerController.SetViewTargetWithBlend` (`GameplayStatics.GetPlayerController` 0) self 0.5 "VTBlend_Linear" 0.0 false)
  (`|PlayMontage` (`self.Mesh`) "/Game/Content/Assets/Animations/AnimationMontages/doll_monster_QTE_Montage.doll_monster_QTE_Montage"
    (:`then`
      (bind _returnvalue (`GameplayStatics.GetActorOfClass` "/Game/Content/Blueprints/Player/BP_FirstPersonCharacter.BP_FirstPersonCharacter_C"))
      (`SceneComponent.SetVisibility` (`/Game/Content/Blueprints/Player/BP_FirstPersonCharacter.SKM_Hands` _returnvalue) false false))
    (:`OnCompleted`
      (`GameplayStatics.SetGlobalTimeDilation` 0.0))))

(event `Attack`
  (`|PlayMontage` (`self.Mesh`) "/Game/Content/Assets/Animations/AnimationMontages/AM_DollAttack.AM_DollAttack"
    (:`OnCompleted`
      _)
    (:`OnInterrupted`
      _))
  (`self.OnAttackEnd`))

(fn `AttackTrace`
  (bind _returnvalue (`SceneComponent.GetSocketLocation` (`self.Mesh`) "DEF-palm_01_R"))
  (if (`self.CanHit`)
    (bind _outhits (`KismetSystemLibrary.SphereTraceMulti` :`Start` _returnvalue :`End` _returnvalue :`Radius` 25.0 :`TraceChannel` "TraceTypeQuery1" :`DrawDebugType` "ForDuration"))
    (for _array_element _outhits
      (bind _succesfull (message `/Game/Content/Blueprints/Management/BPI_Damage.DealDamage` (`.HitActor` (`GameplayStatics.BreakHitResult` _array_element)) 1))
      (if _succesfull
        (`|ExecutionSequence`
          (:`then_0`
            (break))
          (:`then_1`
            (`self.EndAttackTrace`)
            (`self.JumpscareAnim`)))))))

(fn `DamageEnemy`
  (returns (Hit :type Boolean))
  (`self.TakeDamage`)
  (return true))

(fn `DealDamage`
  (params (DamageAmount :type Integer))
  (returns (Succesfull :type Boolean) (RemaningHealth :type Integer))
  (return false 0))

(fn `EndAttackTrace`
  (`KismetSystemLibrary.K2_ClearAndInvalidateTimerHandle` (`self.AttackTraceTimer`))
  (set `self.CanHit` false))

(fn `GetPatrolRoute`
  (returns (PatrolRoute :type "/Game/Content/Blueprints/Enemy/BP_PatrolRoute Object Reference"))
  (return (`self.PatrolRoute`)))

(fn `SetInvestigateValue`
  (params (Value :type "/Game/Content/Blueprints/Data/E_InvestigateValue Enum" :default "NewEnumerator0"))
  (bind _asaic_enemy_base (cast `/Game/Content/Blueprints/Enemy/AIC_EnemyBase` (`AIBlueprintHelperLibrary.GetAIController` self)))
  (switch `/Game/Content/Blueprints/Data/E_InvestigateValue` Value
    (:`NewEnumerator0`
      (`/Game/Content/Blueprints/Enemy/AIC_EnemyBase.SetDefeultPerception` _asaic_enemy_base))
    (:`NewEnumerator1`
      (`/Game/Content/Blueprints/Enemy/AIC_EnemyBase.SetInvestigatePerception` _asaic_enemy_base)))
  (return))

(fn `SetMovementSpeed`
  (params (Speed :type "/Game/Content/Blueprints/Data/E_MovementSpeed Enum" :default "NewEnumerator0"))
  (returns (SpeedValue :type "Float (double-precision)"))
  (bind _output_get (set `CharacterMovementComponent.MaxWalkSpeed` (select `/Game/Content/Blueprints/Data/E_MovementSpeed` Speed :`NewEnumerator1` 100.0 :`NewEnumerator2` 300.0 :`NewEnumerator3` 500.0 :!type "Float (single-precision)") (`self.CharacterMovement`)))
  (return _output_get))

(fn `StartAttackTrace`
  (bind _returnvalue (`KismetSystemLibrary.K2_SetTimerDelegate` (`|CreateDelegate` :!event `AttackTrace`) 0.01 true true))
  (set `self.AttackTraceTimer` _returnvalue)
  (set `self.CanHit` true))

(fn `UserConstructionScript`)