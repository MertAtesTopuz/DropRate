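; Base enemy AI controller that runs the enemy behavior tree and switches its Blackboard state between Passive, Investigate and Attack.
; Perception updates attack a visible, non-hiding player, or investigate heard noises and the location of a hidden or unseen player.
; Attack starts a 2D sound, faded out by the other states.
; Two swappable perception components share one handler, but sense queries only read the default one; damage sensing is stubbed.
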(event `self.ReceivePossess`
  (params (PossessedPawn :type "Pawn Object Reference"))
  (`self.RunBehaviorTree` "/Game/Content/Blueprints/Enemy/BehaviorTree/BT_EnemyBaseTree.BT_EnemyBaseTree")
  (`self.SetStateAsPassive`))

(event `self.DefeultPerception.OnPerceptionUpdated`
  (params (UpdatedActors :type "Array of Actor Object Reference (by ref)"))
  (for _array_element (stale `self.InvestigatePerception.OnPerceptionUpdated` UpdatedActors) :!label _label
    (`|ExecutionSequence`
      (:`then_0`
        (bind _sensed (`self.CanSenseActor` _array_element "NewEnumerator1"))
        (bind _asbp_first_person_character (cast `/Game/Content/Blueprints/Player/BP_FirstPersonCharacter` _array_element))
        (if (and (not (`/Game/Content/Blueprints/Player/BP_FirstPersonCharacter.IsHiding` _asbp_first_person_character)) _sensed)
          (`self.HandleSenseSight` _array_element)
          (else
            (`self.SetStateAsInvestigate` (`self.K2_GetActorLocation` _array_element)))))
      (:`then_1`
        (bind (_sensed_2 _stimulus) (`self.CanSenseActor` _array_element "NewEnumerator2"))
        (if _sensed_2
          (`self.HandleSenseSound` (`.StimulusLocation` (break `AIStimulus` _stimulus)))))
      (:`then_2`
        (bind _sensed_3 (`self.CanSenseActor` null "NewEnumerator3"))
        (if _sensed_3
          _)))))

(event `self.InvestigatePerception.OnPerceptionUpdated`
  (params (UpdatedActors :type "Array of Actor Object Reference (by ref)"))
  (goto _label))

(event `SetDefeultPerception`
  (set `self.InvestigateState` "NewEnumerator0")
  (`ActorComponent.SetActive` (`self.InvestigatePerception`) false false)
  (`ActorComponent.SetActive` (`self.DefeultPerception`) true false))

(event `SetInvestigatePerception`
  (set `self.InvestigateState` "NewEnumerator1")
  (`ActorComponent.SetActive` (`self.DefeultPerception`) false false)
  (`ActorComponent.SetActive` (`self.InvestigatePerception`) true false))

(fn `CanSenseActor`
  (params (Actor :type "Actor Object Reference") (Sense :type "/Game/Content/Blueprints/Data/E_AISense Enum" :default "NewEnumerator0"))
  (returns (Sensed :type Boolean) (Stimulus :type "AIStimulus Structure"))
  (bind _info (`AIPerceptionComponent.GetActorsPerception` (`self.DefeultPerception`) Actor))
  (for _array_element (`.LastSensedStimuli` (break `ActorPerceptionBlueprintInfo` _info))
    (bind _returnvalue (`AIPerceptionSystem.GetSenseClassForStimulus` _array_element))
    (if (== _returnvalue (select `/Game/Content/Blueprints/Data/E_AISense` Sense :`NewEnumerator1` "/Script/AIModule.AISense_Sight" :`NewEnumerator2` "/Script/AIModule.AISense_Hearing" :`NewEnumerator3` "/Script/AIModule.AISense_Damage" :!type "Object Class Reference"))
      (return (`.bSuccessfullySensed` (break `AIStimulus` _array_element)) _array_element))))

(fn `GetCurrentState`
  (returns (State :type "/Game/Content/Blueprints/Data/E_EnemyStates Enum"))
  (return (cast `/Game/Content/Blueprints/Data/E_EnemyStates` (`BlackboardComponent.GetValueAsEnum` (`self.Blackboard`) (`self.StateKey`)))))

(fn `HandleSenseSight`
  (params (NewParam :type "Actor Object Reference"))
  (bind _state (`self.GetCurrentState`))
  (switch `/Game/Content/Blueprints/Data/E_EnemyStates` _state
    (:`NewEnumerator0`
      _)
    (:`NewEnumerator2`
      _))
  (if (== NewParam (`GameplayStatics.GetPlayerCharacter` 0))
    (`self.SetStateAsAttack` NewParam)))

(fn `HandleSenseSound`
  (params (Location :type "Vector Structure"))
  (bind _state (`self.GetCurrentState`))
  (switch `/Game/Content/Blueprints/Data/E_EnemyStates` _state
    (:`NewEnumerator0`
      _)
    (:`NewEnumerator2`
      _))
  (`self.SetStateAsInvestigate` Location))

(fn `SetInvestigateValue`)

(fn `SetStateAsAttack`
  (params (AttackTarget :type "Actor Object Reference"))
  (`BlackboardComponent.SetValueAsEnum` (`self.Blackboard`) (`self.StateKey`) (enumliteral `/Game/Content/Blueprints/Data/E_EnemyStates` "NewEnumerator1"))
  (`BlackboardComponent.SetValueAsObject` (`self.Blackboard`) (`self.AttackTargetKey`) (`GameplayStatics.GetPlayerCharacter` 0))
  (bind _returnvalue (`GameplayStatics.SpawnSound2D` (`self.Sound`) 1.0 1.0 0.0 null))
  (set `self.MainSound` _returnvalue))

(fn `SetStateAsInvestigate`
  (params (Location :type "Vector Structure"))
  (`BlackboardComponent.SetValueAsEnum` (`self.Blackboard`) (`self.StateKey`) (enumliteral `/Game/Content/Blueprints/Data/E_EnemyStates` "NewEnumerator2"))
  (`BlackboardComponent.SetValueAsVector` (`self.Blackboard`) (`self.PointOfInterestKeyName`) Location)
  (bind _mainsound (`self.MainSound`)
    (:`then`
      (`AudioComponent.FadeOut` _mainsound 0.3 0.0 "Linear"))
    (:`else`)))

(fn `SetStateAsPassive`
  (`BlackboardComponent.SetValueAsEnum` (`self.Blackboard`) (`self.StateKey`) (enumliteral `/Game/Content/Blueprints/Data/E_EnemyStates` "NewEnumerator0"))
  (bind _mainsound (`self.MainSound`)
    (:`then`
      (`AudioComponent.FadeOut` _mainsound 0.3 0.0 "Linear"))
    (:`else`)))

(fn `UserConstructionScript`)