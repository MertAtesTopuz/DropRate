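; BP_3DNumericPuzzle is a puzzle actor that opens a numeric padlock interface when interacted with.
; On BeginPlay it limits its scene capture to itself and its child actors, then binds to the interaction result of its BP_Interractable child actor.
; The bound handler creates a WBP_NumericLockUI linked to the BP_NumericLock child actor, adds it to the viewport and plays a start sound, without checking the result.
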(event `self.ReceiveBeginPlay`
  (`SceneCaptureComponent.ShowOnlyActorComponents` (`self.SceneCaptureComponent2D`) self true)
  (bind _asbp_interractable (cast `/Game/Content/Blueprints/Interraction/BP_Interractable` (`ChildActorComponent.ChildActor` (`self.BP_Interractable`))))
  (add `/Game/Content/Blueprints/Interraction/BP_Interractable.InterractionResult` _asbp_interractable (`|CreateDelegate` :!event `BP_3DNumericPuzzle_AutoGenFunc`)))

(fn `BP_3DNumericPuzzle_AutoGenFunc`
  (params (Result :type Boolean))
  (bind _returnvalue (`|CreateWidget` "/Game/Content/Blueprints/UI/WBP_NumericLockUI.WBP_NumericLockUI_C" null (cast `/Game/Content/Blueprints/Interraction/BP_NumericLock` (`ChildActorComponent.ChildActor` (`self.NumericLock`)) :!pure true)))
  (`UserWidget.AddToViewport` _returnvalue 0)
  (`GameplayStatics.PlaySound2D` "/Game/Content/SFXsSenior/PadlockPuzzleBegin_Cue.PadlockPuzzleBegin_Cue" 1.0 1.0 0.0 null null))

(fn `UserConstructionScript`)