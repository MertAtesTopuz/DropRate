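; BP_Throwable is a breakable throwable that creates a noise distraction for enemy AI when it hits something.
; On Hit, it teleports the level's BP_SoundMaker to the hit location, triggers MakeSound and plays a 2D glass-break sound.
; It writes its sphere's location and an investigate state to the blackboard of one BP_EnemyAi found by class, then destroys itself next tick.
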(event `self.ReceiveHit`
  (params (MyComp :type "PrimitiveComponent Object Reference") (Other :type "Actor Object Reference") (OtherComp :type "PrimitiveComponent Object Reference") (bSelfMoved :type Boolean) (HitLocation :type "Vector Structure") (HitNormal :type "Vector Structure") (NormalImpulse :type "Vector Structure") (Hit :type "HitResult Structure (by ref)"))
  (bind _returnvalue (`GameplayStatics.GetActorOfClass` "/Game/Content/Blueprints/Management/BP_SoundMaker.BP_SoundMaker_C"))
  (`self.K2_SetActorLocation` _returnvalue HitLocation false true)
  (`/Game/Content/Blueprints/Management/BP_SoundMaker.MakeSound` _returnvalue)
  (`GameplayStatics.SpawnSound2D` "/Game/Content/Assets/Sounds/SoundWaves/SW_GlassBreak.SW_GlassBreak" 1.0 1.0 0.0 null)
  (bind _returnvalue_2 (`GameplayStatics.GetActorOfClass` "/Game/Content/Blueprints/Enemy/BP_EnemyAi.BP_EnemyAi_C"))
  (bind _returnvalue_3 (`AIBlueprintHelperLibrary.GetBlackboard` _returnvalue_2))
  (`BlackboardComponent.SetValueAsVector` _returnvalue_3 "MoveToLocation" (`SceneComponent.K2_GetComponentLocation` (`self.Sphere`)))
  (`BlackboardComponent.SetValueAsEnum` _returnvalue_3 "State" (`self.InvestigateState`))
  (`KismetSystemLibrary.DelayUntilNextTick`)
  (`self.K2_DestroyActor`))

(fn `UserConstructionScript`)