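; BP_CheckPoint is an indexed checkpoint actor that records player progress.
; When the player character overlaps its box and TriggerBox is set, it calls a SaveGame dispatcher bound to its Save event.
; Save raises the game instance's SpawnIndex only if this Index is higher, then saves the player to a slot.
; On BeginPlay, checkpoints at or below the saved SpawnIndex destroy their BeforeActors.
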(event `self.ReceiveBeginPlay`
  (add `self.SaveGame` (delegate `Save`))
  (bind _asbp_game_instance (cast `/Game/Content/Blueprints/Management/BP_GameInstance` (`GameplayStatics.GetGameInstance`)))
  (if (>= (`/Game/Content/Blueprints/Management/BP_GameInstance.SpawnIndex` _asbp_game_instance) (`self.Index`))
    (for _array_element (`self.BeforeActors`)
      (`self.K2_DestroyActor` _array_element))))

(event `Save`
  (bind _asbp_game_instance (cast `/Game/Content/Blueprints/Management/BP_GameInstance` (`GameplayStatics.GetGameInstance`)))
  (if (> (`self.Index`) (`/Game/Content/Blueprints/Management/BP_GameInstance.SpawnIndex` _asbp_game_instance))
    (set `/Game/Content/Blueprints/Management/BP_GameInstance.SpawnIndex` (`self.Index`) _asbp_game_instance)
    (`/Game/Content/Blueprints/Management/BP_GameInstance.SavePlayerToSlot` _asbp_game_instance)))

(event `self.Box.OnComponentBeginOverlap`
  (params (OverlappedComponent :type "PrimitiveComponent Object Reference") (OtherActor :type "Actor Object Reference") (OtherComp :type "PrimitiveComponent Object Reference") (OtherBodyIndex :type Integer) (bFromSweep :type Boolean) (SweepResult :type "HitResult Structure (by ref)"))
  (if (== OtherActor (`GameplayStatics.GetPlayerCharacter` 0))
    (if (`self.TriggerBox`)
      (`self.SaveGame`))))

(fn `UserConstructionScript`)